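; GF_Bp is a Rank-scaled character Blueprint that answers the human interface queries mostly with neutral defaults, such as not selectable, not dead and no weapon.
; Its working logic stores Sign, Group and Channel in CPBase for side checks, which treat -1 or an inactive state as friendly.
; It also reports remaining summon time and target distance and direction.
; A ground-snap trace helper exists, but its construction-script call is disconnected.
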(event `/Game/Game/Blueprints/Human.iSetSignGroupID`
  (params (Sign :type Integer) (Group :type Integer) (Channel :type Integer))
  (bind _cp_base (`self.CP_Base`))
  (set `/Game/Game/Blueprints/CP_Base.Sign` Sign _cp_base)
  (set `/Game/Game/Blueprints/CP_Base.Group` Group _cp_base)
  (set `/Game/Game/Blueprints/CP_Base.Channel` Channel _cp_base))

(fn `CharaterProperties`
  (returns (Speed :type "Float (double-precision)") (`Can Swim` :type Boolean) (`Can Attk` :type Boolean))
  (return 0.0 false false))

(fn `GetAttkInfo`
  (returns (HasWeapon :type Boolean) (WeaponType :type Integer) (AttkMove :type Integer) (Skill :type "/Game/Game/Enums/ESkillName Enum"))
  (return false 0 0 "NewEnumerator0"))

(fn `getCritChance`
  (returns (percent :type "Float (double-precision)"))
  (return 0.0))

(fn `getSign`
  (returns (sign :type Integer))
  (return (select `bool` (`self.Activated`) :`false` -1 :`true` (`/Game/Game/Blueprints/CP_Base.Sign` (`self.CP_Base`)))))

(fn `iBusy`
  (returns (Fight :type Boolean) (Move :type Boolean))
  (return false false))

(fn `iCannotFocus`
  (returns (result :type Boolean))
  (return false))

(fn `iCheckCurrentAction`
  (params (Action :type "/Game/NewChuAccess/Anim/Action Enum" :default "NewEnumerator0"))
  (returns (Result :type Boolean))
  (return false))

(fn `iCurrentAction`
  (returns (NewParam :type "/Game/NewChuAccess/Anim/Action Enum"))
  (return "NewEnumerator0"))

(fn `iEmotion`
  (returns (Emotion :type "/Game/Game/Blueprints/eEmotion Enum"))
  (return "NewEnumerator0"))

(fn `iGetCurrentAction`
  (returns (NewParam :type "/Game/NewChuAccess/Anim/Action Enum"))
  (return "NewEnumerator0"))

(fn `iGetLevel`
  (returns (level :type Integer))
  (return 0))

(fn `iGetSignGroup`
  (returns (Sign :type Integer) (Group :type Integer) (Channel :type Integer))
  (bind _cp_base (`self.CP_Base`))
  (return (`/Game/Game/Blueprints/CP_Base.Sign` _cp_base) (`/Game/Game/Blueprints/CP_Base.Group` _cp_base) (`/Game/Game/Blueprints/CP_Base.Channel` _cp_base)))

(fn `iGetSummonTimeRemain`
  (returns (TimeRemain :type "Float (double-precision)"))
  (return (`self.SummonTimeRemainning`)))

(fn `iisDied`
  (returns (result :type Boolean))
  (return false))

(fn `iNoAction`
  (returns (NewParam :type Boolean))
  (return false))

(fn `iPlayerControled`
  (params (actor :type "Actor Object Reference"))
  (returns (result :type Boolean))
  (return false))

(fn `iRequestLocation`
  (returns (loc :type "Vector Structure"))
  (return (0.0 0.0 0.0)))

(fn `iSameSide`
  (params (TestActor :type "Actor Object Reference"))
  (returns (result :type Boolean))
  (bind _sign (`/Game/Game/Blueprints/CP_Base.Sign` (`self.CP_Base`)))
  (`/Engine/EditorBlueprintResources/StandardMacros.IsValid` TestActor
    (:`Is Valid`
      (bind _sign_2 (message `/Game/Game/Blueprints/Human.getSign` TestActor))
      (return (or (== _sign_2 _sign) (== _sign_2 -1) (== _sign -1) (not (`self.Activated`)))))
    (:`Is Not Valid`
      (return true))))

(fn `iSelectAble`
  (returns (Success :type Boolean))
  (return false))

(fn `iTargetRelation`
  (params (`New Target` :type "Actor Object Reference") (UseCurrent :type Boolean))
  (returns (Available :type Boolean) (Dist :type "Float (double-precision)") (Direct :type "Vector Structure") (Dot :type "Float (double-precision)"))
  (bind _returnvalue (select `bool` UseCurrent :`false` `New Target` :`true` (`self.EmTarget`)))
  (`/Engine/EditorBlueprintResources/StandardMacros.IsValid` _returnvalue
    (:`Is Valid`
      (bind (_direction _dist _dot) (`/Game/NewChuAccess/Bp/MX_LibA.Mx_Direction` _returnvalue))
      (return true (`KismetMathLibrary.VSize` (* _direction (1.0 1.0 0.0))) _direction _dot))
    (:`Is Not Valid`
      (return false 0.0 (0.0 0.0 0.0) 0.0))))

(fn `PlaceOnGround`
  (params (Z :type "Float (double-precision)"))
  (returns (SweepHitResult :type "HitResult Structure"))
  (bind _returnvalue (`self.K2_GetActorLocation`))
  (bind (_outhit _returnvalue_2) (`KismetSystemLibrary.LineTraceSingleForObjects` _returnvalue (- _returnvalue (`KismetMathLibrary.MakeVector` 0.0 0.0 Z)) (`|MakeArray` "ObjectTypeQuery1" :!type "EObjectTypeQuery Enum")))
  (if _returnvalue_2
    (`self.K2_SetActorLocation` (+ (`.Location` (`GameplayStatics.BreakHitResult` _outhit)) (`KismetMathLibrary.MakeVector` 0.0 0.0 (`CapsuleComponent.GetScaledCapsuleHalfHeight` (`self.CapsuleComponent`))))))
  (return _outhit))

(fn `UpdateAction`
  (returns (action :type "/Game/NewChuAccess/Anim/Action Enum") (UnderWater :type Boolean) (SpeedVector :type "Vector Structure") (Speed :type "Float (double-precision)"))
  (return "NewEnumerator0" false (0.0 0.0 0.0) 0.0))

(fn `UserConstructionScript`
  (`self.SetActorScale3D` (`KismetMathLibrary.Conv_DoubleToVector` (`self.Rank`))))