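; CDTSave is a SaveGame object holding character stats, skills, quest lists, quest items and revive count.
; SetupDefault rolls level-scaled stats with random variance, while helpers handle HP/MP changes, skill checks and quest bookkeeping.
; It saves itself to slots; FLoadSave returns the save loaded by character name or falls back to itself, while LoadLastSave discards its result.
; CalDamage and most interface getters are stubs.
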(event Custom|LoadDefautValue
  (params (level :type Integer))
  (Utilities|SetupDefault level))

(event Custom|AddQuestInventoy
  (params (Item :type EitemName%20Enum) (Remove :type Boolean))
  (bind _questitemlist (Variables|Inventory|GetQuestItemList))
  (if Remove
    (Utilities|Array|RemoveItem _questitemlist Item)
    (else
      (Utilities|Array|AddUnique _questitemlist Item))))

(event Custom|AutoSave
  (SaveGame|SaveGametoSlot self (Variables|Default|GetsaveName)))

(event Custom|NewSave
  (params (name :type Name) (slot :type Integer))
  (SaveGame|SaveGametoSlot self (Utilities|String|ToString(Name) name) slot))

(event Custom|LoadLastSave
  (SaveGame|LoadGamefromSlot (Variables|Default|GetsaveName)))

(event Custom|Add%20Recived%20Quest
  (params (Quest :type EQuestName%20Enum))
  (Utilities|Array|AddUnique (Variables|Quest|GetQuestRecivedList) Quest))

(event Custom|UpdateData
  (CallFunction|LoadDefautValue (Variables|Rank|Getlevel)))

(event Custom|Add%20Finished%20Quest
  (params (Quest :type EQuestName%20Enum))
  (Utilities|Array|AddUnique (Variables|Quest|GetQuestFinishedList) Quest)
  (Utilities|Array|RemoveItem (Variables|Quest|GetQuestRecivedList) Quest))

(event Custom|AddRevive
  (params (Num :type Integer))
  (Variables|Charater|SetReviveNum (Math|Integer|Clamp(Integer) (+ (Variables|Charater|GetReviveNum) Num) 0 99)))

(event EventIAddquestInventory
  (params (QuestItem :type EitemName%20Enum :default "NewEnumerator1") (Remove :type Boolean))
  (CallFunction|AddQuestInventoy QuestItem Remove))

(fn HpPercent
  (return (/ (Variables|baseic|Gethp) (Variables|baseic|GetMaxHp))))

(fn MpPercent
  (return (/ (Variables|baseic|Getmp) (Variables|baseic|GetMaxMp))))

(fn FLoadSave
  (bind _returnvalue (SaveGame|LoadGamefromSlot (Variables|Charater|GetCharaterName)))
  (bind _ascdtsave (Utilities|Casting|CastToCDTSave _returnvalue)
    (:then
      (LocalVariables|SetNewLocalVar_0 _ascdtsave))
    (:CastFailed
      (LocalVariables|SetNewLocalVar_0 self)))
  (return (LocalVariables|GetNewLocalVar_0)))

(fn CalDamage)

(fn IsKillAvailable
  (params (skill :type ESkillName%20Enum))
  (return (Utilities|Array|ContainsItem (Variables|Skill|GetSkillList) skill)))

(fn IsCanCastSkill
  (params (Skill :type Integer))
  (bind _result (CallFunction|IsKillAvailable (Utilities|Enum|ByteToEnumESkillName (Math|Conversions|ToByte(Integer) Skill))))
  (return _result))

(fn UseMp
  (params (Cost :type Float%20%28single-precision%29))
  (if (>= (- (Variables|baseic|Getmp) Cost) 0.0)
    (Variables|baseic|Setmp (- (Variables|baseic|Getmp) Cost)))
  (return (>= (- (Variables|baseic|Getmp) Cost) 0.0) (Variables|baseic|Getmp)))

(fn HpChange
  (params (Hp :type Float%20%28single-precision%29))
  (return (Math|Float|Clamp(Float) (+ (Variables|baseic|Gethp) Hp) 0.0 (Variables|baseic|GetMaxHp))))

(fn AddMHp
  (params (Mp :type Float%20%28single-precision%29) (Hp :type Float%20%28single-precision%29))
  (bind _output_get (Variables|baseic|Setmp (Math|Float|Clamp(Float) (+ Mp (Variables|baseic|Getmp)) 0.0 (Variables|baseic|GetMaxMp))))
  (bind _output_get_2 (Variables|baseic|Sethp (Math|Float|Clamp(Float) (+ (Variables|baseic|Gethp) Hp) 0.0 (Variables|baseic|GetMaxHp))))
  (return _output_get _output_get_2))

(fn ICurrentLevelDisplayName
  (return ""))

(fn IGetCurrentQuest
  (return "NewEnumerator0"))

(fn IGetLang
  (return "NewEnumerator0"))

(fn IgettextBylang
  (params (lang :type Elang%20Enum :default "NewEnumerator0"))
  (return ""))

(fn IisNewGame
  (return false))

(fn ILoadProfile
  (params (name :type String))
  (return 0))

(fn IMapLevelActived
  (params (MapName :type EMapName%20Enum :default "NewEnumerator0") (InList :type Array%20of%20EMapName%20Enums))
  (return false))

(fn IPlayerName
  (return ""))

(fn IsMapActive
  (params (Map%20name :type EMapName%20Enum :default "NewEnumerator0"))
  (return false))

(fn ITutorialShow
  (return false))