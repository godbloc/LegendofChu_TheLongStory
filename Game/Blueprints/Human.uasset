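; Human is a Blueprint Interface, judging by its body-less functions, defining a shared contract for human-like characters.
; Movement calls cover input axes, swimming, flight, move-to, follow, flee and physics.
; Combat calls span melee, ranged and thrown attacks, damage, crits, freeze, death and respawn.
; Query and setter calls expose action state, animation data, AI class, level, XP and sign/group allegiance, so callers need no concrete class.
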(fn `AtTrackTo`
  (params (position :type "Vector Structure") (speed :type "Float (double-precision)")))

(fn `CanDamage`
  (params (active :type Boolean) (damage :type "Float (double-precision)")))

(fn `CharaterProperties`
  (returns (Speed :type "Float (double-precision)") (`Can Swim` :type Boolean) (`Can Attk` :type Boolean))
  (return 0.0 false false))

(fn `feedbackHit`
  (params (`hitted ` :type "Actor Object Reference") (damage :type "Float (double-precision)") (crit :type Boolean)))

(fn `GetAttkInfo`
  (returns (HasWeapon :type Boolean) (WeaponType :type Integer) (AttkMove :type Integer) (Skill :type "/Game/Game/Enums/ESkillName Enum"))
  (return false 0 0 "NewEnumerator0"))

(fn `getCritChance`
  (returns (percent :type "Float (double-precision)"))
  (return 0.0))

(fn `GetHumanStatus`
  (params (Status :type "/Game/Game/Blueprints/EhumanStatus Enum")))

(fn `GetHurt`
  (params (Damage :type "Float (double-precision)") (Cause :type "Actor Object Reference") (multi :type "Float (double-precision)")))

(fn `getSign`
  (returns (sign :type Integer))
  (return 0))

(fn `HookToActor`
  (params (actor :type "Actor Object Reference") (active :type Boolean)))

(fn `iAction`
  (params (value :type "/Game/NewChuAccess/Anim/Action Enum") (ref :type "Actor Object Reference")))

(fn `IAddvelocity`
  (params (Vel :type "Vector Structure") (Scalar :type "Float (double-precision)")))

(fn `iAEvent`)

(fn `iBoostSpeed`
  (params (Scale :type "Float (double-precision)") (Dur :type "Float (double-precision)")))

(fn `iBusy`
  (returns (Fight :type Boolean) (Move :type Boolean))
  (return false false))

(fn `iCannotFocus`
  (returns (result :type Boolean))
  (return false))

(fn `iCapScreen`)

(fn `iChangeAiClass`
  (params (`Ai class` :type "AIController Class Reference")))

(fn `iCheckCurrentAction`
  (params (Action :type "/Game/NewChuAccess/Anim/Action Enum"))
  (returns (Result :type Boolean))
  (return false))

(fn `iChooseTypeAndSign`
  (params (`Actor Type` :type Integer) (sign :type Integer)))

(fn `iCurrentAction`
  (returns (NewParam :type "/Game/NewChuAccess/Anim/Action Enum"))
  (return "NewEnumerator0"))

(fn `iDeath`)

(fn `iDEvent`)

(fn `iEmotion`
  (returns (Emotion :type "/Game/Game/Blueprints/eEmotion Enum"))
  (return "NewEnumerator0"))

(fn `iEquipWeapon`
  (params (Weapon :type "/Game/MainCharater/Weapon/Bp/WP_BaseClass Object Reference")))

(fn `iFight`
  (params (action :type "/Game/NewChuAccess/Anim/Action Enum") (range :type Boolean) (dist :type "Float (double-precision)") (Hook :type Boolean)))

(fn `iFloater`)

(fn `iFlyup`
  (params (axis :type "Float (double-precision)")))

(fn `iFocusTarget`
  (params (Target :type "Actor Object Reference")))

(fn `iFollowActor`
  (params (des :type "Actor Object Reference") (r1 :type "Float (double-precision)") (r2 :type "Float (double-precision)")))

(fn `iFreeze`
  (params (inTime :type "Float (double-precision)") (slowTime :type "Float (double-precision)")))

(fn `iGetCurrentAction`
  (returns (NewParam :type "/Game/NewChuAccess/Anim/Action Enum"))
  (return "NewEnumerator0"))

(fn `iGetLevel`
  (returns (level :type Integer))
  (return 0))

(fn `iGetSignGroup`
  (returns (Sign :type Integer) (Group :type Integer) (Channel :type Integer))
  (return 0 0 0))

(fn `iGoForWard`
  (params (scale :type "Float (double-precision)")))

(fn `iGoup`
  (params (Scale :type "Float (double-precision)")))

(fn `iisDied`
  (returns (result :type Boolean))
  (return false))

(fn `iKeyRelease`
  (params (key :type "/Game/Game/Enums/EButtonName Enum") (Time :type "Float (double-precision)")))

(fn `iLevelUp`
  (params (value :type Integer)))

(fn `iMoveForwar`
  (params (axis :type "Float (double-precision)")))

(fn `iMoveRight`
  (params (axis :type "Float (double-precision)")))

(fn `iMovetoLocation`
  (params (Location :type "Vector Structure") (Limit :type "Float (double-precision)") (rapit :type Boolean) (FaceTo :type Boolean)))

(fn `iNoAction`
  (returns (NewParam :type Boolean))
  (return false))

(fn `iPlayerControled`
  (params (actor :type "Actor Object Reference"))
  (returns (result :type Boolean))
  (return false))

(fn `iPlayPhysic`
  (params (Duration :type "Float (double-precision)") (Gravity :type "Vector Structure")))

(fn `iRequestLocation`
  (returns (loc :type "Vector Structure"))
  (return (0.0 0.0 0.0)))

(fn `iRequireAllAnimationNeed`
  (params (Transform :type "Transform Structure") (MoveSpeed :type "Vector Structure") (UseWeapon :type Boolean) (SpaceState :type "/Game/Game/Enums/ECdtSpaceState Enum") (`Attack Num` :type Integer) (Action :type "/Game/NewChuAccess/Anim/Action Enum") (WeaponType :type Integer)))

(fn `iRespawn`
  (params (Owner :type "Actor Object Reference")))

(fn `iRestoreState`)

(fn `iRotateBack`)

(fn `iRunAway`
  (params (FromTarget :type "Actor Object Reference") (KeepDistance :type "Float (double-precision)")))

(fn `iSameSide`
  (params (TestActor :type "Actor Object Reference"))
  (returns (result :type Boolean))
  (return false))

(fn `iSelectAble`
  (returns (Success :type Boolean))
  (return false))

(fn `iSetaction`
  (params (NewParam :type "/Game/NewChuAccess/Anim/Action Enum")))

(fn `iSetlevel`
  (params (level :type Integer)))

(fn `iSetRQLocation`
  (params (loc :type "Vector Structure")))

(fn `iSetSignGroupID`
  (params (Sign :type Integer) (Group :type Integer) (Channel :type Integer)))

(fn `iSetSkin`
  (params (Mat :type "MaterialInstance Object Reference") (InTime :type "Float (double-precision)")))

(fn `iSetVelocity`
  (params (vel :type "Vector Structure")))

(fn `iSEvent`)

(fn `iTalk`
  (params (text :type String) (delay :type "Float (double-precision)")))

(fn `iTargetRelation`
  (params (`New Target` :type "Actor Object Reference") (UseCurrent :type Boolean))
  (returns (Available :type Boolean) (Dist :type "Float (double-precision)") (Direct :type "Vector Structure") (Dot :type "Float (double-precision)"))
  (return false 0.0 (0.0 0.0 0.0) 0.0))

(fn `iThrow`
  (params (Aim :type Boolean) (Fire :type Boolean)))

(fn `iTurnRight`
  (params (axis :type "Float (double-precision)") (case :type Integer)))

(fn `iTurnUp`
  (params (axis :type "Float (double-precision)") (case :type Integer)))

(fn `iUnFreeze`)

(fn `iWEvent`)

(fn `iXPUp`
  (params (value :type Integer)))

(fn `LookAt`
  (params (`Point View` :type "Vector Structure")))

(fn `MelleAttk`
  (params (`Has Weapon` :type Boolean) (`weapon Id` :type Integer) (`Attk move` :type Integer)))

(fn `RangeAttack`)

(fn `SetAction`
  (params (action :type "/Game/NewChuAccess/Anim/Action Enum")))

(fn `StopAttk`)

(fn `toggleSwimMode`
  (params (`Water location` :type "Vector Structure")))

(fn `UnderWater`
  (params (`New Active` :type Boolean) (`Water location` :type "Vector Structure")))

(fn `UpdateAction`
  (returns (action :type "/Game/NewChuAccess/Anim/Action Enum") (UnderWater :type Boolean) (SpeedVector :type "Vector Structure") (Speed :type "Float (double-precision)"))
  (return "NewEnumerator0" false (0.0 0.0 0.0) 0.0))