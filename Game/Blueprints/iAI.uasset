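; iAI is a Blueprint Interface declaring the contract for commanding and querying AI agents, with no logic of its own.
; Movement and mission calls cover pathing to locations, mission paths, tracking or focusing actors, returning home, waiting, dismissal and mission status.
; Combat and control calls cover enemy detection, current and lost target queries, control checks and capture release.
; An activation call takes an AI class and tree to switch in new AI behavior.
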(fn `iActiveNewAi`
  (params (`Ai Class` :type "AIController Class Reference") (`Ai Tree` :type "BehaviorTree Object Reference") (`Ai Tb` :type "BlackboardData Object Reference")))

(fn `iAIPathToLocation`
  (params (Location :type "Vector Structure") (Status :type "/Game/NewChuAccess/Bp/ECdtFollowStatus Enum")))

(fn `iAISetMission`
  (params (Loc :type "Vector Structure") (Stat :type "/Game/Game/AITree/EMissionStatus Enum")))

(fn `iBackHome`)

(fn `iCheckControled`
  (params (A :type "Actor Object Reference"))
  (returns (Result :type Boolean) (Current :type "Actor Object Reference"))
  (return false null))

(fn `iCurrentTarget`
  (returns (Actor :type "Actor Object Reference") (Available :type Boolean))
  (return null false))

(fn `iDetectEnemy`
  (params (Max :type "Float (double-precision)") (Min :type "Float (double-precision)") (ByClass :type "Actor Class Reference") (Stat :type "/Game/NewChuAccess/Monster_Character/EEnemyStat Enum"))
  (returns (Actors :type "Array of Actor Object Reference"))
  (return))

(fn `iDismiss`)

(fn `iDoMission`
  (params (Next :type Boolean)))

(fn `iFocusToActor`
  (params (Actor :type "Actor Object Reference")))

(fn `iFollowMissionPath`
  (params (Path :type "SplineComponent Object Reference") (ForceMove :type Boolean)))

(fn `iGetMissionStat`
  (returns (NewParam :type "/Game/Game/AITree/EMissionStatus Enum"))
  (return "NewEnumerator0"))

(fn `iGetTarget`
  (returns (Target :type "Actor Object Reference") (Available :type Boolean))
  (return null false))

(fn `iLostTarget`
  (returns (Died :type Boolean) (Faraway :type Boolean))
  (return false false))

(fn `ireachGoal`
  (params (Dist :type "Float (double-precision)"))
  (returns (NewParam :type Boolean))
  (return false))

(fn `iReleaseCapture`
  (params (Act :type "Actor Object Reference") (Accept :type Boolean)))

(fn `iTrackToActor`
  (params (Actor :type "Actor Object Reference") (Dist :type "Float (double-precision)"))
  (returns (Closed :type Boolean))
  (return false))

(fn `iWaitingfor`)