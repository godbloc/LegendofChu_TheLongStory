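; Flag actor that links to another flag of its class through NextFlag, with a sphere sized from Radius at construction.
; DetectNearFlag gathers flags using NearActors with a 300-to-MaxDistance range and, when RandomLoc is set, randomly picks one that does not point back to it.
; GenNextFlag instead picks any flag in the level at random, possibly itself, as its not-same-location check is unconnected.
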(event `DetectNearFlag`
  (bind _returnvalue (`GameplayStatics.GetObjectClass` self))
  ;[1 1 1] DetectNearFlag
  (`GameplayStatics.GetAllActorsOfClass` _returnvalue)
  (bind (_result _count) (`/Game/common/GXFuncs_v9.NearActors` self _returnvalue 300.0 (`self.maxDistance`)))
  (for _array_element _result
    (if (`self.RandomLoc`)
      (bind _asflag_bp (cast `/Game/Blueprints/FlagBp` (`KismetArrayLibrary.Array_Get` _result (`KismetMathLibrary.RandomIntegerInRange` 0 _count))))
      (if (!= (`/Game/Blueprints/FlagBp.NextFlag` _asflag_bp) self)
        (`/Engine/EditorBlueprintResources/StandardMacros.IsValid` _array_element
          (:`Is Valid`
            (set `self.NextFlag` _asflag_bp)
            (break)))))))

(fn `GenNextFlag`
  (bind _outactors (`GameplayStatics.GetAllActorsOfClass` "FlagBp_C"))
  (if true
    (set `self.NextFlag` (`KismetArrayLibrary.Array_Get` _outactors (`KismetMathLibrary.RandomIntegerInRange` 0 (- (`KismetArrayLibrary.Array_Length` _outactors) 1))))
    (else
      (`self.GenNextFlag`))))

(fn `UserConstructionScript`
  (`SphereComponent.SetSphereRadius` (`self.Sphere`) (`self.Radius`) true))