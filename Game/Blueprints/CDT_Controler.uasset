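; CDT_Controler is an input controller that relays player movement and combat input to the player character through interface messages.
; Axis events forward up, forward and right values, while Pressed actions send throw (aim and fire) and fight messages with fixed arguments.
; The forward axis also accumulates its value into TimePress while nonzero, resets it at zero, and sends the running total alongside the current value.
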(event `InputAxis|TMoveUp`
  (params (AxisValue :type "Float (single-precision)"))
  (message `/Game/Game/Blueprints/Human.iFlyup` (`GameplayStatics.GetPlayerCharacter` 0) AxisValue))

(event `InputAxis|TmoveForWard`
  (params (AxisValue :type "Float (single-precision)"))
  (bind _returnvalue (`GameplayStatics.GetPlayerCharacter` 0))
  (bind _timepress (`self.TimePress`))
  (message `/Game/Game/Blueprints/Human.iMoveForwar` _returnvalue AxisValue)
  ;[1 1 1] Time Press
  (if (!= AxisValue 0.0)
    (set `self.TimePress` (+ _timepress AxisValue))
    (else
      (set `self.TimePress` 0.0)))
  (message `/Game/Game/Interface/iPlayer.iAxisInputPress` _returnvalue _timepress AxisValue))

(event `InputAxis|TMoveRight`
  (params (AxisValue :type "Float (single-precision)"))
  (message `/Game/Game/Blueprints/Human.iMoveRight` (`GameplayStatics.GetPlayerCharacter` 0) AxisValue))

(event `InputAction|ThrowFire`
  (params (Key :type "Key Structure" :default "AnyKey"))
  (:`Pressed`
    (message `/Game/Game/Blueprints/Human.iThrow` (`GameplayStatics.GetPlayerCharacter` 0) true true)))

(event `InputAction|Fight`
  (params (Key :type "Key Structure" :default "AnyKey"))
  (:`Pressed`
    (message `/Game/Game/Blueprints/Human.iFight` (`GameplayStatics.GetPlayerCharacter` 0) "NewEnumerator3" false 10.0 false)))

(fn `UserConstructionScript`)