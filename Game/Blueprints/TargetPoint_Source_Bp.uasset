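; Destructible troop spawn point that sends AI units along a spline path behind a moving flag, with a touch-toggled widget.
; On timed ticks or a create command it spawns units within a capacity that refills as they die, assigning team sign, group and path or end-point mission.
; The flag troop advances by allied headcount and signals path completion at the end.
; Heavy hits drain HP and reward the attacker.
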(event `/Game/Game/Blueprints/iGAME.iAddWidget`
  (params (Wg :type "UserWidget Object Reference"))
  ;[1 1 1] Iset Widget
  (`WidgetComponent.SetWidget` (`self.WgControl`) Wg))

(event `ToggleShowIcon` :!signature `self.OnInputTouchBegin`
  (params (FingerIndex :type "ETouchIndex Enum") (TouchedActor :type "Actor Object Reference"))
  ;[1 1 1] Touch Enter
  (bind _isa (`/Engine/EditorBlueprintResources/StandardMacros.FlipFlop`)
    (:`A`
      _)
    (:`B`
      _))
  (`SceneComponent.SetHiddenInGame` (`self.WgControl`) _isa false)
  (`GameplayStatics.SpawnEmitterAtLocation` "/Game/ParticleSystem/PaticularEffect/Effects/Aura/growup_Fire.growup_Fire" (`self.K2_GetActorLocation`)))

(event `self.ReceiveBeginPlay`
  ;[1 1 1] BeginPlay
  (message `/Game/Game/Blueprints/iAI.iFollowMissionPath` (`self.Flag`) (`self.Spline`) false)
  (message `/Game/Game/Blueprints/Human.iSetSignGroupID` (`ChildActorComponent.ChildActor` (`self.Flag`)) (`self.sign`) (`self.GroupId`) 0)
  (add `self.OnInputTouchBegin` (delegate `ToggleShowIcon`))
  (add `self.OnInputTouchLeave` (delegate `ToggleShowIcon`))
  (message `/Game/Game/Blueprints/iGAME.iSetParent` (`ChildActorComponent.ChildActor` (`self.Flag`)) self (`self.GroupId`)))

(event `ESpawnAI`
  (params (`Actor Type` :type Integer))
  ;[1 1 1] Spawn Ai
  (if (> (`self.CapCount`) 0)
    (bind _returnvalue (`AIBlueprintHelperLibrary.SpawnAIFromClass` "/Game/NewChuAccess/Bp/Cdt_Dummy_New.Cdt_Dummy_New_C" "/Game/Game/AITree/BT_SimpleMoveTree.BT_SimpleMoveTree" (+ (`self.Offset`) (0.0 0.0 100.0)) (struct) true))
    (`/Engine/EditorBlueprintResources/StandardMacros.IsValid` _returnvalue
      (:`Is Valid`
        (set `Actor.Tags` (`|MakeArray` "HasMission" :!type "Name") _returnvalue)
        (set `self.Count` (+ (`self.Count`) 1))
        (set `self.CapCount` (- (`self.CapCount`) 1))
        (if (`self.Attack`)
          (message `/Game/Game/Blueprints/Human.iChooseTypeAndSign` _returnvalue `Actor Type` (`self.sign`))
          (message `/Game/Game/Blueprints/iAI.iFollowMissionPath` _returnvalue (`self.Spline`) true)
          (else
            (message `/Game/Game/Blueprints/iAI.iAISetMission` _returnvalue (`self.RequestLoc`) "NewEnumerator0")))
        (`KismetArrayLibrary.Array_Add` (`self.Actors`) _returnvalue)
        (message `/Game/Game/Blueprints/Human.iSetSignGroupID` _returnvalue (`self.sign`) (`self.GroupId`) 0)))))

(event `ECheckAvailable`
  (bind _actors (`self.Actors`))
  ;[1 1 1] Check Available
  (if (> (`KismetArrayLibrary.Array_Length` _actors) 0)
    (for _array_element _actors
      (`/Engine/EditorBlueprintResources/StandardMacros.IsValid` _array_element
        (:`Is Not Valid`
          (`KismetArrayLibrary.Array_RemoveItem` _actors _array_element)
          (`self.ECheckAvailable`)
          (`/Engine/EditorBlueprintResources/StandardMacros.IncrementInt` (`self.CapCount`)))))))

(event `/Game/Game/Blueprints/iGAME.iSetPathLength`
  (params (NewParam :type "Float (single-precision)") (realative :type Boolean))
  (bind _returnvalue (`SplineComponent.GetSplineLength` (`self.Spline`)))
  ;[1 1 1] Drive To location
  (if realative
    (set `self.PathLength` (`KismetMathLibrary.FClamp` (+ (`self.PathLength`) NewParam) 0.0 _returnvalue))
    (else
      (set `self.PathLength` (`KismetMathLibrary.FClamp` NewParam 0.0 _returnvalue)))))

(event `EDriveToLocation`
  (bind _spline (`self.Spline`))
  (bind _pathlength (`self.PathLength`))
  (bind _flag (`self.Flag`))
  (bind _pathlength_2 (`self.PathLength`))
  (bind _speed (`self.Speed`))
  ;[1 1 1] Drive To location
  (bind _ascdt_flag_troop (cast `/Game/Game/Blueprints/Cdt_FlagTroop` (`ChildActorComponent.ChildActor` _flag)))
  (bind (_has_actors _num) (`/Game/Game/Blueprints/Cdt_FlagTroop.GetAllyActorCount` _ascdt_flag_troop))
  (if _has_actors
    (set `self.PathLength` (+ _pathlength_2 (* _num _speed)))
    (else
      (set `self.PathLength` (+ _pathlength_2 (/ _speed 5.0)))))
  (`SceneComponent.K2_SetRelativeLocation` _flag (`SplineComponent.GetLocationAtDistanceAlongSpline` _spline _pathlength "Local") false true)
  (if (>= _pathlength (`SplineComponent.GetSplineLength` _spline))
    (`self.DFinishPath`)
    (`self.SetActorTickEnabled` false)))

(event `self.ReceiveTick`
  (params (DeltaSeconds :type "Float (single-precision)"))
  ;[1 1 1] Tick
  (`|ExecutionSequence`
    (:`then_0`
      (`KismetSystemLibrary.Delay` (`self.SpawnTime`))
      (`self.ECheckAvailable`)
      (message `/Game/Game/Blueprints/iGAME.iSetTroopForm` (`ChildActorComponent.ChildActor` (`self.Flag`)) (`self.Actors`) 0)
      (if (`self.AuToSpawn`)
        (`self.ESpawnAI` (`KismetMathLibrary.RandomIntegerInRange` 0 5))))
    (:`then_1`
      (`self.EDriveToLocation`))))

(event `self.ReceiveAnyDamage`
  (params (Damage :type "Float (single-precision)") (DamageType :type "DamageType Object Reference") (InstigatedBy :type "Controller Object Reference") (DamageCauser :type "Actor Object Reference"))
  ;[1 1 1] Damage
  (`/Engine/EditorBlueprintResources/StandardMacros.IsValid` DamageCauser
    (:`Is Valid`
      (if (> Damage 100.0)
        (bind _output_get (set `self.Hp` (- (`self.Hp`) Damage)))
        (`GameplayStatics.SpawnEmitterAtLocation` "/Game/ParticleSystem/PaticularEffect/Effects/Aura/growup_Fire.growup_Fire" (`self.K2_GetActorLocation`) (struct))
        (if (< _output_get 0.0)
          (`self.K2_DestroyActor`)
          (message `/Game/Game/Blueprints/Human.iLevelUp` DamageCauser 1)
          (else
            (message `/Game/Game/Blueprints/Human.iXPUp` DamageCauser 1)))))))

(event `/Game/MenuWidget/iWidget.iActivate`
  (params (ref :type "Actor Object Reference") (value :type Integer) (Cmd :type "/Game/Game/Structs/IconCommandStruct Structure"))
  (bind (_img _bkg _command _ecmd _cname _value) (break `/Game/Game/Structs/IconCommandStruct` Cmd))
  (switch `/Game/Game/Enums/ECommandType` _ecmd
    (:`NewEnumerator4`
      (`self.ESpawnAI` _value))))

(fn `CharaterProperties`
  (returns (Speed :type "Float (double-precision)") (`Can Swim` :type Boolean) (`Can Attk` :type Boolean))
  (return 0.0 false false))

(fn `GetAttkInfo`
  (returns (HasWeapon :type Boolean) (WeaponType :type Integer) (AttkMove :type Integer) (Skill :type "/Game/Game/Enums/ESkillName Enum"))
  (return false 0 0 "NewEnumerator0"))

(fn `getCritChance`
  (returns (percent :type "Float (double-precision)"))
  (return 0.0))

(fn `getSign`
  (returns (sign :type Integer))
  (return (`self.sign`)))

(fn `iBusy`
  (returns (Fight :type Boolean) (Move :type Boolean))
  (return false false))

(fn `iCannotFocus`
  (returns (result :type Boolean))
  (return false))

(fn `iCheckCurrentAction`
  (params (Action :type "/Game/NewChuAccess/Anim/Action Enum" :default "NewEnumerator0"))
  (returns (Result :type Boolean))
  (return false))

(fn `iCurrentAction`
  (returns (NewParam :type "/Game/NewChuAccess/Anim/Action Enum"))
  (return "NewEnumerator0"))

(fn `iCurrentLevelDisplayName`
  (returns (name :type String))
  (return ""))

(fn `iEmotion`
  (returns (Emotion :type "/Game/Game/Blueprints/eEmotion Enum"))
  (return "NewEnumerator0"))

(fn `iGetCurrentAction`
  (returns (NewParam :type "/Game/NewChuAccess/Anim/Action Enum"))
  (return "NewEnumerator0"))

(fn `iGetCurrentGameSave`
  (params (reload :type Boolean) (PlayerId :type Integer))
  (returns (Game :type "/Game/Game/Blueprints/GameSave Object Reference") (Player :type "/Game/Game/Blueprints/CDTSave Object Reference"))
  (return null null))

(fn `iGetCurrentQuest`
  (returns (QuestName :type "/Game/Game/Blueprints/QuestData/EQuestName Enum"))
  (return "NewEnumerator0"))

(fn `iGetLang`
  (returns (result :type "/Game/Game/Blueprints/Cdt_lang Enum"))
  (return "NewEnumerator0"))

(fn `iGetLevel`
  (returns (level :type Integer))
  (return 0))

(fn `iGetSignGroup`
  (returns (Sign :type Integer) (Group :type Integer) (Channel :type Integer))
  (return (`self.sign`) (`self.GroupId`) 0))

(fn `igettextBylang`
  (params (lang :type "/Game/Game/Blueprints/Elang Enum" :default "NewEnumerator0"))
  (returns (result :type String))
  (return ""))

(fn `iisDied`
  (returns (result :type Boolean))
  (return false))

(fn `iisNewGame`
  (returns (value :type Boolean))
  (return false))

(fn `iLoadProfile`
  (params (name :type String))
  (returns (save :type "/Game/Game/Blueprints/CDTSave Object Reference"))
  (return null))

(fn `iMapLevelActived`
  (params (MapName :type "/Game/Game/Enums/EMapName Enum" :default "NewEnumerator0") (InList :type "Array of /Game/Game/Enums/EMapName Enum (by ref)"))
  (returns (Actived :type Boolean))
  (return false))

(fn `iNoAction`
  (returns (NewParam :type Boolean))
  (return false))

(fn `iPlayerControled`
  (params (actor :type "Actor Object Reference"))
  (returns (result :type Boolean))
  (return false))

(fn `iPlayerName`
  (returns (`Player name` :type String))
  (return ""))

(fn `iRequestLocation`
  (returns (loc :type "Vector Structure"))
  (return (0.0 0.0 0.0)))

(fn `iSameSide`
  (params (TestActor :type "Actor Object Reference"))
  (returns (result :type Boolean))
  (`/Engine/EditorBlueprintResources/StandardMacros.IsValid` TestActor
    (:`Is Valid`
      (bind _sign (message `/Game/Game/Blueprints/Human.getSign` TestActor))
      (return (== _sign (`self.sign`))))
    (:`Is Not Valid`
      (return true))))

(fn `iSelectAble`
  (returns (Success :type Boolean))
  (return false))

(fn `IsMapActive`
  (params (`Map name` :type "/Game/Game/Enums/EMapName Enum" :default "NewEnumerator0"))
  (returns (result :type Boolean))
  (return false))

(fn `iTargetRelation`
  (params (`New Target` :type "Actor Object Reference") (UseCurrent :type Boolean))
  (returns (Available :type Boolean) (Dist :type "Float (double-precision)") (Direct :type "Vector Structure") (Dot :type "Float (double-precision)"))
  (return false 0.0 (0.0 0.0 0.0) 0.0))

(fn `iTutorialShow`
  (returns (Result :type Boolean))
  (return false))

(fn `UpdateAction`
  (returns (action :type "/Game/NewChuAccess/Anim/Action Enum") (UnderWater :type Boolean) (SpeedVector :type "Vector Structure") (Speed :type "Float (double-precision)"))
  (return "NewEnumerator0" false (0.0 0.0 0.0) 0.0))

(fn `UserConstructionScript`
  (bind _spline (`self.Spline`))
  (bind _output_get (set `self.Offset` (`SplineComponent.GetLocationAtSplinePoint` _spline 0 "World")))
  (set `self.RequestLoc` (`SplineComponent.GetLocationAtSplinePoint` _spline (- (`SplineComponent.GetNumberOfSplinePoints` _spline) 1) "World"))
  (`SceneComponent.K2_SetWorldLocation` (`self.Flag`) _output_get false false))