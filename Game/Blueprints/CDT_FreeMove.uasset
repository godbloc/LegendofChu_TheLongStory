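; Touch player controller for selecting and commanding units, with a cursor, control widget and spawned pick icon.
; A touch traces under the finger: same-sign selectables become the controlled pawn, others get focused, and bare locations receive a move order on a quick repeat tap.
; Dragging pans the view target, Zoom toggles zoom and restore, and FreeMove gates turn axes.
; Commands travel as interface messages; most implemented interface functions are default stubs.
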(event `/Game/Game/Blueprints/iAI.iReleaseCapture`
  (params (Act :type "Actor Object Reference") (Accept :type Boolean))
  ;[1 1 1] Comment
  (if Accept
    (bind _result (`self.iCheckControled` Act))
    (if _result
      (`self.ReleaseActor`))))

(event `ReleaseActor`
  ;[1 1 1] Release Actor
  (set `self.ActorPawn` null))

(event `TakeControl`
  (params (RapidPress :type Boolean) (FastMove :type Boolean) (`Move to` :type Boolean) (CurrentTouchLoc :type "Vector Structure"))
  (bind _actorpawn (`self.ActorPawn`))
  ;[1 1 1] Tak Control to Actor
  (`/Engine/EditorBlueprintResources/StandardMacros.IsValid` _actorpawn
    (:`Is Valid`
      (if `Move to`
        (message `/Game/Game/Blueprints/iAI.iAISetMission` _actorpawn CurrentTouchLoc "NewEnumerator0")))))

(event `self.ReceiveBeginPlay`
  ;[1 1 1] BeginPlay
  (bind _returnvalue (`|SpawnActorFromClass` "/Game/Game/DropItem/Actor_icon.Actor_icon_C" (`KismetMathLibrary.MakeTransform` (0.0 0.0 0.0)) "AlwaysSpawn" "OverrideRootScale"))
  (set `self.PickActorWidget` _returnvalue)
  (set `self.bShowMouseCursor` true)
  (bind _returnvalue_2 (`|CreateWidget` "/Game/MenuWidget/Widget_control/Wg_control2.Wg_control2_C"))
  (bind _output_get (set `self.WgControl` _returnvalue_2))
  (`UserWidget.AddToViewport` _output_get 0))

(event `self.ReceiveTick`
  (params (DeltaSeconds :type "Float (single-precision)")))

(event `InputAxis|TurnLeft`
  (params (AxisValue :type "Float (single-precision)"))
  ;[1 1 1] Comment
  (if (`self.FreeMove`)
    (message `/Game/Game/Blueprints/Human.iTurnRight` (`GameplayStatics.GetPlayerPawn` 0) AxisValue 0)))

(event `InputAxis|turnUp`
  (params (AxisValue :type "Float (single-precision)"))
  ;[1 1 1] Comment
  (if (`self.FreeMove`)
    (message `/Game/Game/Blueprints/Human.iTurnUp` (`GameplayStatics.GetPlayerPawn` 0) AxisValue 0)))

(event `RapitPress`
  ;[1 1 1] Comment
  (message `/Game/Game/Blueprints/Human.iBoostSpeed` (`self.ActorPawn`) 2.0 1.0))

(event `InputTouch`
  (params (Location :type "Vector Structure") (FingerIndex :type "ETouchIndex Enum"))
  (bind _returnvalue (`self.GetViewTarget`))
  (bind _actorpawn (`self.ActorPawn`))
  (bind _returnvalue_2 (- (`self.LastTouchLoc`) Location))
  (:`Pressed`
    ;[1 1 1] Touching
    (bind (_new_time _delta _returnvalue_3) (`self.TouchTime` 0.5))
    (set `self.ControlMode` 0)
    (bind (_success _new_pawn _location) (`self.SelectPawnFromLocation` Location))
    (if _success
      (`self.SwitChControl` _new_pawn _location
        (:`New Actor Pawn`
          (message `/Game/Game/Blueprints/iCamera.iSnapViewToLocation` _returnvalue _location :!label _label)
          (`GameplayStatics.SpawnEmitterAtLocation` "/Game/ParticleSystem/PaticularEffect/Effects/Aura/Pa_PickIndicator.Pa_PickIndicator" _location))
        (:`Focus Enemy`
          (message `/Game/Game/Blueprints/iAI.iFocusToActor` _actorpawn _new_pawn))
        (:`Only Location`
          (set `self.LastTouchLoc` Location)
          (`/Engine/EditorBlueprintResources/StandardMacros.IsValid` _actorpawn
            (:`Is Valid`
              (if _returnvalue_3
                (message `/Game/Game/Blueprints/iAI.iAISetMission` _actorpawn _location "NewEnumerator0")
                (`GameplayStatics.SpawnEmitterAtLocation` "/Game/Game/Pa_PickLocation.Pa_PickLocation" _location))))))))
  (:`Released`
    (set `self.ControlMode` 1)
    (set `self.LastTouchLoc` Location)
    (goto _label))
  (:`Moved`
    (set `self.ControlMode` 2)
    (if (> (`KismetMathLibrary.VSize` _returnvalue_2) 15.0)
      (message `/Game/Game/Blueprints/iCamera.iPanning` _returnvalue (`KismetMathLibrary.ClampVectorSize` _returnvalue_2 0.0 10.0))
      (set `self.LastTimeSecond` (`GameplayStatics.GetRealTimeSeconds`)))))

(event `InputAction|Zoom`
  (params (Key :type "Key Structure" :default "AnyKey"))
  (bind _returnvalue (`self.GetViewTarget`))
  (bind _actorpawn (`self.ActorPawn`))
  ;[1 1 1] Zoom
  (:`Pressed`
    (`/Engine/EditorBlueprintResources/StandardMacros.FlipFlop`
      (:`A`
        (message `/Game/Game/Blueprints/iCamera.iSmoothZoom` _returnvalue 1000.0 true)
        (`/Engine/EditorBlueprintResources/StandardMacros.IsValid` _actorpawn
          (:`Is Valid`
            (message `/Game/Game/Blueprints/iGAME.iSnapViewtoTarget` _returnvalue _actorpawn true))))
      (:`B`
        (message `/Game/Game/Blueprints/iCamera.iCameraRestore` _returnvalue true)))))

(event `/Game/Game/Blueprints/iControler.iSendCommand`
  (params (CMID :type Integer) (Message :type String) (Data :type "Actor Object Reference")))

(fn `CharaterProperties`
  (returns (Speed :type "Float (double-precision)") (`Can Swim` :type Boolean) (`Can Attk` :type Boolean))
  (return 0.0 false false))

(fn `GetAttkInfo`
  (returns (HasWeapon :type Boolean) (WeaponType :type Integer) (AttkMove :type Integer) (Skill :type "/Game/Game/Enums/ESkillName Enum"))
  (return false 0 0 "NewEnumerator0"))

(fn `getCritChance`
  (returns (percent :type "Float (double-precision)"))
  (return 0.0))

(fn `getSign`
  (returns (sign :type Integer))
  (return (`self.Sign`)))

(fn `iBusy`
  (returns (Fight :type Boolean) (Move :type Boolean))
  (return false false))

(fn `iCannotFocus`
  (returns (result :type Boolean))
  (return false))

(fn `iCheckControled`
  (params (A :type "Actor Object Reference"))
  (returns (Result :type Boolean) (Current :type "Actor Object Reference"))
  (bind _actorpawn (`self.ActorPawn`))
  (return (== _actorpawn A) _actorpawn))

(fn `iCheckCurrentAction`
  (params (Action :type "/Game/NewChuAccess/Anim/Action Enum" :default "NewEnumerator0"))
  (returns (Result :type Boolean))
  (return false))

(fn `iCurrentAction`
  (returns (NewParam :type "/Game/NewChuAccess/Anim/Action Enum"))
  (return "NewEnumerator0"))

(fn `iCurrentLevelDisplayName`
  (returns (name :type String))
  (return ""))

(fn `iCurrentTarget`
  (returns (Actor :type "Actor Object Reference") (Available :type Boolean))
  (return null false))

(fn `iDetectEnemy`
  (params (Max :type "Float (double-precision)") (Min :type "Float (double-precision)") (ByClass :type "Actor Class Reference") (Stat :type "/Game/NewChuAccess/Monster_Character/EEnemyStat Enum" :default "NewEnumerator0"))
  (returns (Actors :type "Array of Actor Object Reference"))
  (return (`|MakeArray` null :!type "Actor Object Reference")))

(fn `iEmotion`
  (returns (Emotion :type "/Game/Game/Blueprints/eEmotion Enum"))
  (return "NewEnumerator0"))

(fn `iGetCurrentAction`
  (returns (NewParam :type "/Game/NewChuAccess/Anim/Action Enum"))
  (return "NewEnumerator0"))

(fn `iGetCurrentQuest`
  (returns (QuestName :type "/Game/Game/Blueprints/QuestData/EQuestName Enum"))
  (return "NewEnumerator0"))

(fn `iGetLang`
  (returns (result :type "/Game/Game/Blueprints/Cdt_lang Enum"))
  (return "NewEnumerator0"))

(fn `iGetLevel`
  (returns (level :type Integer))
  (return 0))

(fn `iGetMissionStat`
  (returns (NewParam :type "/Game/Game/AITree/EMissionStatus Enum"))
  (return "NewEnumerator0"))

(fn `iGetSignGroup`
  (returns (Sign :type Integer) (Group :type Integer) (Channel :type Integer))
  (return 0 0 0))

(fn `iGetTarget`
  (returns (Target :type "Actor Object Reference") (Available :type Boolean))
  (return null false))

(fn `igettextBylang`
  (params (lang :type "/Game/Game/Blueprints/Elang Enum" :default "NewEnumerator0"))
  (returns (result :type String))
  (return ""))

(fn `iisDied`
  (returns (result :type Boolean))
  (return false))

(fn `iisNewGame`
  (returns (value :type Boolean))
  (return false))

(fn `iLoadProfile`
  (params (name :type String))
  (returns (save :type "/Game/Game/Blueprints/CDTSave Object Reference"))
  (return null))

(fn `iLostTarget`
  (returns (Died :type Boolean) (Faraway :type Boolean))
  (return false false))

(fn `iMapLevelActived`
  (params (MapName :type "/Game/Game/Enums/EMapName Enum" :default "NewEnumerator0") (InList :type "Array of /Game/Game/Enums/EMapName Enum (by ref)"))
  (returns (Actived :type Boolean))
  (return false))

(fn `iNoAction`
  (returns (NewParam :type Boolean))
  (return false))

(fn `iPlayerControled`
  (params (actor :type "Actor Object Reference"))
  (returns (result :type Boolean))
  (return false))

(fn `iPlayerName`
  (returns (`Player name` :type String))
  (return ""))

(fn `ireachGoal`
  (params (Dist :type "Float (double-precision)"))
  (returns (NewParam :type Boolean))
  (return false))

(fn `iRequestLocation`
  (returns (loc :type "Vector Structure"))
  (return (0.0 0.0 0.0)))

(fn `iSameSide`
  (params (TestActor :type "Actor Object Reference"))
  (returns (result :type Boolean))
  (return false))

(fn `iSelectAble`
  (returns (Success :type Boolean))
  (return false))

(fn `IsMapActive`
  (params (`Map name` :type "/Game/Game/Enums/EMapName Enum" :default "NewEnumerator0"))
  (returns (result :type Boolean))
  (return false))

(fn `iTargetRelation`
  (params (`New Target` :type "Actor Object Reference") (UseCurrent :type Boolean))
  (returns (Available :type Boolean) (Dist :type "Float (double-precision)") (Direct :type "Vector Structure") (Dot :type "Float (double-precision)"))
  (return false 0.0 (0.0 0.0 0.0) 0.0))

(fn `iTrackToActor`
  (params (Actor :type "Actor Object Reference") (Dist :type "Float (double-precision)"))
  (returns (Closed :type Boolean))
  (return false))

(fn `iTutorialShow`
  (returns (Result :type Boolean))
  (return false))

(fn `SelectPawnFromLocation`
  (params (Loc :type "Vector Structure"))
  (returns (Success :type Boolean) (`New Pawn` :type "Actor Object Reference") (Location :type "Vector Structure") (Moveable :type Boolean))
  (bind (_hitresult _returnvalue) (`self.GetHitResultUnderFingerForObjects` "Touch1" (`|MakeArray` "ObjectTypeQuery3" "ObjectTypeQuery4" "ObjectTypeQuery1" :!type "EObjectTypeQuery Enum") false))
  (bind (_bblockinghit _binitialoverlap _time _location _impactpoint _normal _impactnormal _physmat _hitactor) (`GameplayStatics.BreakHitResult` _hitresult))
  (bind _returnvalue_2 (`KismetSystemLibrary.DoesImplementInterface` _hitactor "/Game/Game/Blueprints/iSelectAble.iSelectAble_C"))
  (if _returnvalue
    (message `/Game/Game/Blueprints/Human.iSelectAble` _hitactor)
    (if _returnvalue_2
      (return true _hitactor _location false)
      (else
        (return true null _location _returnvalue_2)))
    (else
      (return false null Loc false))))

(fn `SetTouchByIndex`
  (params (NewParam :type "ETouchIndex Enum") (NewParam1 :type "Vector Structure"))
  (switch `ETouchIndex` NewParam))

(fn `TouchTime`
  (params (CheckTime :type "Float (double-precision)"))
  (returns (`New time` :type "Float (double-precision)") (Delta :type "Float (double-precision)") (ReturnValue :type Boolean))
  (bind _returnvalue (`GameplayStatics.GetRealTimeSeconds`))
  (bind _output_get (set `self.Deltatime` (- _returnvalue (`self.LastTimeSecond`))))
  (bind _output_get_2 (set `self.LastTimeSecond` _returnvalue))
  (return _output_get_2 _output_get (<= _output_get CheckTime)))

(fn `UpdateAction`
  (returns (action :type "/Game/NewChuAccess/Anim/Action Enum") (UnderWater :type Boolean) (SpeedVector :type "Vector Structure") (Speed :type "Float (double-precision)"))
  (return "NewEnumerator0" false (0.0 0.0 0.0) 0.0))

(fn `UserConstructionScript`)