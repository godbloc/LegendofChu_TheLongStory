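; iGAME is a Blueprint interface declaring game-wide calls, with empty bodies or default returns only.
; It covers saving and loading of games, levels and player profiles, plus new-game start, language, player name and level display name.
; Further calls handle widgets and focus, quests and quest inventory, tutorials and map activation checks.
; A few gameplay hooks cover view snapping to a target, parenting, path length and troop formations.
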(fn `iAddFinishQuest`
  (params (Quest :type "/Game/Game/Blueprints/QuestData/EQuestName Enum")))

(fn `iAddquestInventory`
  (params (QuestItem :type "/Game/Game/DropItem/EitemName Enum") (Remove :type Boolean)))

(fn `iAddReciveQuest`
  (params (Quest :type "/Game/Game/Blueprints/QuestData/EQuestName Enum")))

(fn `iAddToSavelist`
  (params (saveName :type String)))

(fn `iAddWidget`
  (params (Wg :type "UserWidget Object Reference")))

(fn `iClearAllSave`)

(fn `iCurrentLevelDisplayName`
  (returns (name :type String))
  (return ""))

(fn `iGetCurrentQuest`
  (returns (QuestName :type "/Game/Game/Blueprints/QuestData/EQuestName Enum"))
  (return "NewEnumerator0"))

(fn `iGetLang`
  (returns (result :type "/Game/Game/Blueprints/Cdt_lang Enum"))
  (return "NewEnumerator0"))

(fn `igettextBylang`
  (params (lang :type "/Game/Game/Blueprints/Elang Enum"))
  (returns (result :type String))
  (return ""))

(fn `iisNewGame`
  (returns (value :type Boolean))
  (return false))

(fn `iLoadCurrentLevel`)

(fn `iLoadGame`)

(fn `iLoadPlayerProfile`
  (params (Player :type "Actor Object Reference")))

(fn `iLoadProfile`
  (params (name :type String))
  (returns (save :type "/Game/Game/Blueprints/CDTSave Object Reference"))
  (return null))

(fn `iMapLevelActived`
  (params (MapName :type "/Game/Game/EMapName Enum") (InList :type "Array of /Game/Game/EMapName Enum"))
  (returns (Actived :type Boolean))
  (return false))

(fn `iPlayerName`
  (returns (`Player name` :type String))
  (return ""))

(fn `iRemoveWidget`
  (params (wg :type "UserWidget Object Reference")))

(fn `iSaveCurrentlevel`
  (params (levelname :type String)))

(fn `iSaveGame`)

(fn `iSavePlayerProfile`
  (params (Profile :type "SaveGame Object Reference")))

(fn `iSetCurrentLevelDisplayName`
  (params (Name :type String)))

(fn `iSetFocusWidget`)

(fn `iSetLang`
  (params (lang :type "/Game/Game/Blueprints/Cdt_lang Enum")))

(fn `iSetParent`
  (params (Parent :type "Actor Object Reference") (Value :type Integer)))

(fn `iSetPathLength`
  (params (NewParam :type "Float (double-precision)") (realative :type Boolean)))

(fn `iSetPlayerName`
  (params (NewName :type String)))

(fn `iSetShowTut`
  (params (Active :type Boolean))
  (return))

(fn `iSetTroopForm`
  (params (Actors :type "Array of Actor Object Reference") (FormID :type Integer)))

(fn `iShowTutorial`
  (params (Index :type Integer)))

(fn `IsMapActive`
  (params (`Map name` :type "/Game/Game/EMapName Enum"))
  (returns (result :type Boolean))
  (return false))

(fn `iSnapViewtoTarget`
  (params (Target :type "Actor Object Reference") (KeepRotation :type Boolean)))

(fn `iStartNewGame`)

(fn `iTutorialShow`
  (returns (Result :type Boolean))
  (return false))

(fn `iUpdateQuestList`
  (params (QList :type "Array of /Game/Game/Blueprints/QuestData/EQuestName Enum")))

(fn `LoadLastLevel`)