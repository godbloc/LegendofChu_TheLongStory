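; CDTgameMode is a game mode Blueprint that declares start overrides and "i"-prefixed, interface-style queries for game state.
; The queries cover saves and profiles, current quest and level name, language and localized text, active maps, player name, new-game status and tutorial display.
; Every graph is an empty stub returning a default value, including ChoosePlayerStart and ReadyToStartMatch, so no working logic appears here.
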(fn `ChoosePlayerStart`
  (params (Player :type "Controller Object Reference"))
  (returns (ReturnValue :type "Actor Object Reference"))
  (return null))

(fn `iCurrentLevelDisplayName`
  (returns (name :type String))
  (return ""))

(fn `iGetCurrentGameSave`
  (params (reload :type Boolean) (PlayerId :type Integer))
  (returns (Game :type "/Game/Game/Blueprints/GameSave Object Reference") (Player :type "/Game/Game/Blueprints/CDTSave Object Reference"))
  (return null null))

(fn `iGetCurrentQuest`
  (returns (QuestName :type "/Game/Game/Blueprints/QuestData/EQuestName Enum"))
  (return "NewEnumerator0"))

(fn `iGetLang`
  (returns (result :type "/Game/Game/Blueprints/Cdt_lang Enum"))
  (return "NewEnumerator0"))

(fn `igettextBylang`
  (params (lang :type "/Game/Game/Blueprints/Elang Enum" :default "NewEnumerator0"))
  (returns (result :type String))
  (return ""))

(fn `iisNewGame`
  (returns (value :type Boolean))
  (return false))

(fn `iLoadProfile`
  (params (name :type String))
  (returns (save :type "/Game/Game/Blueprints/CDTSave Object Reference"))
  (return null))

(fn `iMapLevelActived`
  (params (MapName :type "/Game/Game/Enums/EMapName Enum" :default "NewEnumerator0") (InList :type "Array of /Game/Game/Enums/EMapName Enum (by ref)"))
  (returns (Actived :type Boolean))
  (return false))

(fn `iPlayerName`
  (returns (`Player name` :type String))
  (return ""))

(fn `IsMapActive`
  (params (`Map name` :type "/Game/Game/Enums/EMapName Enum" :default "NewEnumerator0"))
  (returns (result :type Boolean))
  (return false))

(fn `iTutorialShow`
  (returns (Result :type Boolean))
  (return false))

(fn `ReadyToStartMatch`
  (returns (ReturnValue :type Boolean))
  (return false))

(fn `UserConstructionScript`)