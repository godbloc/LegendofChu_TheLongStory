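; GridBp is a decal-drawn spawn grid that places AI pawns on its cells up to a capacity.
; Construction scales the decal to rows and columns, traces it to the ground and caches node centers.
; BeginPlay adds a widget per node with a random actor type; IActivate spawns at a given node.
; In Auto mode, Tick fills empty nodes with random types; spawns inherit CPBase sign/group/channel and decrement CapCount.
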(event EventIActivate
  (params (ref :type Actor%20Object%20Reference) (value :type Integer) (Cmd :type Icon%20Command%20Struct%20Structure))
  ;[1 1 1] Activate
  (CallFunction|SpawnatNodeIndex value "/Game/NewChuAccess/Bp/Cdt_Dummy_New.Cdt_Dummy_New_C" "/Game/Game/AITree/BT_SimpleMoveTree.BT_SimpleMoveTree" (.Value (Utilities|Struct|BreakIconCommandStruct Cmd))))

(event EventBeginPlay
  ;[1 1 1] begin
  (CallFunction|MakeIconList))

(event EventTick
  (params (DeltaSeconds :type Float%20%28single-precision%29))
  ;[1 1 1] Tick
  (if (Variables|Default|GetAuto)
    (bind (_returnvalue _index) (CallFunction|AutoSpawnActor (Math|Random|RandomIntegerinRange 0 (Utilities|Array|Length (Variables|Default|GetActorTypeList)))))
    (Utilities|Array|SetArrayElem (Variables|Default|GetActors) _index _returnvalue true)))

(fn ConstructionScript
  (bind _returnvalue (Rendering|Material|CreateDynamicMaterialInstance (Variables|Default|GetDecal) :!class /Script/Engine.DecalComponent))
  (Variables|Default|SetGridMaterial _returnvalue)
  (CallFunction|CalculateGrid)
  (bind (_outhit _success) (Utilities|MxTracetoGround 1e+04 "TraceTypeQuery3" "ForOneFrame"))
  (if _success
    (Transformation|SetWorldLocation (Variables|Default|GetDecal) (.Location (Collision|BreakHitResult _outhit)) false false)
    (CallFunction|MakeNodes)))

(fn CalculateGrid
  (bind _row (Variables|Default|GetRow))
  (bind _col (Variables|Default|GetCol))
  (bind _returnvalue (Math|Conversions|ToFloat(Integer) _row))
  (bind _returnvalue_2 (Math|Conversions|ToFloat(Integer) _col))
  (Rendering|Material|SetVectorParameterValue (Variables|Default|GetGridMaterial) "Tilling" (Utilities|Struct|MakeLinearColor _returnvalue _returnvalue_2 0.0 0.0) :!class /Script/Engine.MaterialInstanceDynamic)
  (Variables|Default|SetSizes (Math|Vector|MakeVector 1e+02 (* _returnvalue_2 (Variables|Default|GetSizeY)) (* _returnvalue (Variables|Default|GetSizeX))))
  (Transformation|SetRelativeScale3D (Variables|Default|GetDecal) (Variables|Default|GetSizes)))

(fn GetSelectNodeLocation
  (params (Row :type Integer) (Col :type Integer))
  (return (Utilities|Array|Get(acopy) (Variables|Default|GetNodes) (- (* Row Col) 1))))

(fn MakeNodes
  (bind _sizex (Variables|Default|GetSizeX))
  (bind _sizey (Variables|Default|GetSizeY))
  (bind _row (Variables|Default|GetRow))
  (bind _col (Variables|Default|GetCol))
  (bind _decal (Variables|Default|GetDecal))
  (bind _returnvalue (Transformation|GetWorldLocation _decal))
  (bind _returnvalue_2 (- _row 1))
  (bind _returnvalue_3 (- _col 1))
  (bind (_x _y _z) (Math|Vector|BreakVector _returnvalue))
  (Utilities|Array|Clear (Variables|Default|GetNodes))
  (for _index (range 0 _returnvalue_3)
    (for _index_2 (range 0 _returnvalue_2)
      (Utilities|Array|Add (Variables|Default|GetNodes) (Math|Vector|MakeVector (- (+ _x (* (* _sizex 2.0) (Math|Conversions|ToFloat(Integer) _index_2))) (* _sizex (Math|Conversions|ToFloat(Integer) _returnvalue_2))) (- (+ _y (* (* _sizey 2.0) (Math|Conversions|ToFloat(Integer) _index))) (* _sizey (Math|Conversions|ToFloat(Integer) _returnvalue_3))) _z))
      (Rendering|Debug|DrawDebugBox (Math|Vector|MakeVector (- (+ _x (* (* _sizex 2.0) (Math|Conversions|ToFloat(Integer) _index_2))) (* _sizex (Math|Conversions|ToFloat(Integer) _returnvalue_2))) (- (+ _y (* (* _sizey 2.0) (Math|Conversions|ToFloat(Integer) _index))) (* _sizey (Math|Conversions|ToFloat(Integer) _returnvalue_3))) _z) "22.000000,22.000000,22.000000" "(R=0.910000,G=0.771879,B=0.377650,A=1.000000)" "0, 0, 0" 0.01 1.0))))

(fn GetSelectNodefromLocation
  (params (Loc :type Vector))
  (bind (_x _y) (Math|Vector|BreakVector Loc))
  (bind (_result _index) (CallFunction|XNearestPoint (Variables|Default|GetNodes) (Math|Vector|MakeVector _x _y (.Z (Math|Vector|BreakVector (Transformation|GetWorldLocation (Variables|Default|GetDecal))))) 1e+02))
  (return _result _index))

(fn GetNodeUnderFinger
  (params (Pawn :type Pawn%20Class%20Reference) (BehaviorTree :type Behavior%20Tree%20Object%20Reference) (Spawned :type Boolean))
  (bind _returnvalue (Game|GetPlayerController 0))
  (bind (_hitresult _returnvalue_2) (Class|PlayerController|GetHitResultUnderFingerbyChannel _returnvalue "Touch1" "TraceTypeQuery1" true))
  (if _returnvalue_2
    (bind (_newparam _index) (CallFunction|GetSelectNodefromLocation (.Location (Collision|BreakHitResult _hitresult))))
    (if Spawned
      (Utilities|IsValid (Utilities|Array|Get(acopy) (Variables|Default|GetActors) _index)
        (:Is%20Valid
          _)
        (:Is%20Not%20Valid
          (Rendering|Debug|DrawDebugBox _newparam "111.000000,111.000000,111.000000" "(R=0.204454,G=0.212683,B=0.910000,A=1.000000)" "0, 0, 0" 1.0 1.0)
          (if (> _index 0)
            (CallFunction|SpawnatNodeIndex _index Pawn BehaviorTree (Math|Random|RandomIntegerinRange 0 9))))))
    (return _newparam _index)
    (else
      (return "0, 0, 0" -1))))

(fn SpawnatNodeIndex
  (params (Index :type Integer) (PawnClass :type Pawn%20Class%20Reference) (BehaviorTree :type Behavior%20Tree%20Object%20Reference) (Actor%20Type :type Integer))
  (bind _cp_base (Variables|Default|GetCP_Base))
  (bind _sign (Variables|/Game/Game/Blueprints/CP_Base.CP_Base_C|GetSign _cp_base))
  (if (> (Variables|Default|GetCapCount) 0)
    (bind _returnvalue (AI|SpawnAIFromClass PawnClass BehaviorTree (+ (Utilities|Array|Get(acopy) (Variables|Default|GetNodes) Index) "0, 0,100.000000") "0, 0, 0" true))
    (Utilities|Array|SetArrayElem (Variables|Default|GetActors) Index _returnvalue true)
    (Class|Human|IChooseTypeandSign(Message) _returnvalue Actor%20Type _sign)
    (Class|Human|ISetSignGroupID(Message) _returnvalue _sign (Variables|/Game/Game/Blueprints/CP_Base.CP_Base_C|GetGroup _cp_base) (Variables|/Game/Game/Blueprints/CP_Base.CP_Base_C|GetChannel _cp_base))
    (bind _output_get (Variables|Default|SetCapCount (- (Variables|Default|GetCapCount) 1)))
    (Actor|SetOwner _returnvalue self)
    (return _returnvalue _output_get)
    (else
      (return 0 0))))

(fn AutoSpawnActor
  (params (Actor%20Type :type Integer))
  (for _index (range 0 (Utilities|Array|LastIndex (Variables|Default|GetNodes)))
    (Utilities|IsValid (Utilities|Array|Get(acopy) (Variables|Default|GetActors) _index)
      (:Is%20Not%20Valid
        (bind _returnvalue (CallFunction|SpawnatNodeIndex _index "/Game/NewChuAccess/Bp/Cdt_Dummy_New.Cdt_Dummy_New_C" "/Game/Game/AITree/BT_SimpleMoveTree.BT_SimpleMoveTree" Actor%20Type))
        (return _returnvalue _index))))
  (return 0 0))

(fn MakeIconList
  (bind _actortypelist (Variables|Default|GetActorTypeList))
  (for (_array_element _array_index) (Variables|Default|GetNodes)
    (bind _returnvalue (AddComponent|AddWidgetComponent false (Math|Transform|MakeTransform _array_element)))
    (Transformation|SetWorldLocation _returnvalue _array_element false false)
    (Class|IWidget|IChangeRefActor(Message) (UserInterface|GetUserWidgetObject _returnvalue) self (Utilities|Array|Get(acopy) _actortypelist (Math|Random|RandomIntegerinRange 0 (Utilities|Array|LastIndex _actortypelist))) (Math|Conversions|ToFloat(Integer) _array_index))
    (Development|SetHiddeninGame _returnvalue (not (Variables|Default|GetShow)) false)))

(fn GetRemainActors
  (bind _actors (Variables|Default|GetActors))
  (for (_array_element _array_index) _actors
    (Utilities|IsValid _array_element
      (:Is%20Not%20Valid
        (Utilities|Array|RemoveIndex _actors _array_index))))
  (return (Utilities|Array|Length _actors) (Variables|Default|GetCapCount)))

(fn RemoveActor
  (params (Pawn :type Pawn%20Object%20Reference) (RestoreCap :type Boolean))
  (Utilities|Array|RemoveItem (Variables|Default|GetActors) Pawn)
  (if RestoreCap
    (Math|Integer|IncrementInt (Variables|Default|GetCapCount))))

(fn CharaterProperties
  (return 0.0 false false))

(fn GetAttkInfo
  (return false 0 0 "NewEnumerator0"))

(fn GetCritChance
  (return 0.0))

(fn GetSign
  (return 0))

(fn IBusy
  (return false false))

(fn ICannotFocus
  (return false))

(fn ICheckCurrentAction
  (params (Action :type Action%20Enum :default "NewEnumerator0"))
  (return false))

(fn ICurrentAction
  (return "NewEnumerator0"))

(fn IEmotion
  (return "NewEnumerator0"))

(fn IGetCurrentAction
  (return "NewEnumerator0"))

(fn IGetLevel
  (return 0))

(fn IGetSignGroup
  (return 0 0 0))

(fn IisDied
  (return false))

(fn INoAction
  (return false))

(fn IPlayerControled
  (params (actor :type Actor%20Object%20Reference))
  (return false))

(fn IRequestLocation
  (return "0, 0, 0"))

(fn ISameSide
  (params (TestActor :type Actor%20Object%20Reference))
  (return false))

(fn ISelectAble
  (return false))

(fn ITargetRelation
  (params (New%20Target :type Actor%20Object%20Reference) (UseCurrent :type Boolean))
  (return false 0.0 "0, 0, 0" 0.0))

(fn UpdateAction
  (return "NewEnumerator0" false "0, 0, 0" 0.0))