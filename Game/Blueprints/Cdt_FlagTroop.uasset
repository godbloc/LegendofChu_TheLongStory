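; Troop rally flag that gathers same-sign, same-group units inside its radius sphere.
; Its ally count sends units to focus the last enemy attacker, or to mission points placed around the flag by sine/cosine.
; Hits shorten the linked parent's path length; enemy hits also pass on half damage and award the attacker XP.
; Touch toggles its widget, activation forwards to the parent, and most other interface functions are stubs.
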(event Custom|ToggleShowIcon
  (params (FingerIndex :type ETouchIndex%20Enum) (TouchedActor :type Actor%20Object%20Reference))
  (bind _output_get (Variables|Default|SetShow (not (Variables|Default|GetShow))))
  (CallFunction|ShowWidget _output_get)
  (Utilities|FlowControl|Delay 5.0)
  (if (Variables|Default|GetShow)
    (CallFunction|ShowWidget false)))

(event Custom|ShowWidget
  (params (Hide :type Boolean))
  (Development|SetHiddeninGame (Variables|Default|GetWgControl) Hide false)
  (Effects|SpawnEmitteratLocation "/Game/ParticleSystem/PaticularEffect/Effects/Aura/Pa_PickIndicator.Pa_PickIndicator" (Transformation|GetActorLocation)))

(event EventISetParent
  (params (Parent :type Actor%20Object%20Reference) (Value :type Integer))
  (Variables|Default|SetaffectActor Parent)
  (Variables|Default|SetGroupID Value))

(event EventISetTroopForm
  (params (Actors :type Array%20of%20Actor%20Object%20References) (FormID :type Integer))
  (bind _returnvalue (Transformation|GetActorLocation))
  (bind _radius (Variables|Default|GetRadius))
  (bind (_x _y _z) (Math|Vector|BreakVector _returnvalue))
  (bind _returnvalue_2 (* _radius 0.8))
  (switch int FormID
    (:Default
      _)
    (:0
      _))
  (for (_array_element _array_index) Actors
    (Utilities|IsValid _array_element
      (:Is%20Valid
        (Class|IAI|IAISetMission(Message) _array_element (Math|Vector|MakeVector (|(((R*0.800000)*(sin(a)))+X) _returnvalue_2 (* (/ (Math|Conversions|ToFloat(Integer) (Utilities|Array|Length Actors)) 3.14) (Math|Conversions|ToFloat(Integer) _array_index)) _x) (|(((R*0.800000)*(cos(a)))+Y) _returnvalue_2 (* (/ (Math|Conversions|ToFloat(Integer) (Utilities|Array|Length Actors)) 3.14) (Math|Conversions|ToFloat(Integer) _array_index)) _y) _z) "NewEnumerator0")))))

(event Game|Damage|EventAnyDamage
  (params (Damage :type Float%20%28single-precision%29) (DamageType :type Damage%20Type%20Object%20Reference) (InstigatedBy :type Controller%20Object%20Reference) (DamageCauser :type Actor%20Object%20Reference))
  (bind _affectactor (Variables|Default|GetaffectActor))
  (bind _result (CallFunction|ISameSide DamageCauser))
  (if _result
    (Class|IGAME|ISetPathLength(Message) _affectactor -5.0 true)
    (else
      (Game|Damage|ApplyDamage _affectactor (/ Damage 2.0) 0 0)
      (Class|IGAME|ISetPathLength(Message) _affectactor (* Damage -1.0) true)
      (Variables|Default|SetImpotantEnemy DamageCauser)
      (Class|Human|IXPUp(Message) DamageCauser 5))))

(event EventISetSignGroupID
  (params (Sign :type Integer) (Group :type Integer) (Channel :type Integer))
  (Variables|Default|SetSign Sign)
  (Variables|Default|SetGroupID Group)
  (Variables|Default|SetChannel Channel))

(event EventIActivate
  (params (ref :type Actor%20Object%20Reference) (value :type Integer) (Cmd :type Icon%20Command%20Struct%20Structure))
  (Class|IWidget|IActivate(Message) (Variables|Default|GetaffectActor) ref value Cmd)
  (Utilities|MxShowMessage (Utilities|String|ToString(Integer) value) "(R=0.825000,G=0.068555,B=0.084969,A=1.000000)"))

(event EventBeginPlay
  (EventDispatchers|BindEventtoOnInputTouchBegin (delegate Custom|ToggleShowIcon))
  (Default|CreateCommandby (Variables|Default|GetCp_Commander) false))

(event EventIFollowMissionPath
  (params (Path :type Spline%20Component%20Object%20Reference) (ForceMove :type Boolean)))

(event EventIAddWidget
  (params (Wg :type User%20Widget%20Object%20Reference))
  (UserInterface|SetWidget (Variables|Default|GetWgControl) Wg))

(fn ConstructionScript
  (Components|Sphere|SetSphereRadius (Variables|Default|GetRegione) (Variables|Default|GetRadius) true))

(fn GenNextFlag
  (bind _outactors (Actor|GetAllActorsOfClass "/Game/Game/Blueprints/FlagBp.FlagBp_C"))
  (if true
    (Variables|Default|SetNextFlag (Utilities|Array|Get(acopy) _outactors (Math|Random|RandomIntegerinRange 0 (- (Utilities|Array|Length _outactors) 1))))
    (else
      (CallFunction|GenNextFlag))))

(fn GetAllyActorCount
  (bind _aforms (LocalVariables|GetAForms))
  (bind _impotantenemy (Variables|Default|GetImpotantEnemy))
  (bind _regione (Variables|Default|GetRegione))
  (bind _overlappingactors (Collision|GetOverlappingActors _regione "/Game/NewChuAccess/Bp/Cdt_Dummy_New.Cdt_Dummy_New_C" :!class /Script/Engine.PrimitiveComponent))
  (for _array_element _overlappingactors
    (bind (_sign _group) (Class|Human|IGetSignGroup(Message) _array_element))
    (if (and (== (Variables|Default|GetGroupID) _group) (== _sign (Variables|Default|GetSign)))
      (Math|Integer|IncrementInt (LocalVariables|Getfnum)
        (:%20%20
          (Utilities|Array|Add _aforms _array_element)
          (Utilities|IsValid _impotantenemy
            (:Is%20Valid
              (Class|IAI|IFocustoActor(Message) _array_element _impotantenemy))
            (:Is%20Not%20Valid
              (CallFunction|ISetTroopForm _aforms)))))
      (elif (not (== _sign (Variables|Default|GetSign)))
        (LocalVariables|Setfnum 0))))
  (return (> (LocalVariables|Getfnum) 0) (LocalVariables|Getfnum) _overlappingactors))

(fn AddtoForm)

(fn CharaterProperties
  (return 0.0 false false))

(fn GetAttkInfo
  (return false 0 0 "NewEnumerator0"))

(fn GetCritChance
  (return 0.0))

(fn GetSign
  (return (Variables|Default|GetSign)))

(fn IBusy
  (return false false))

(fn ICannotFocus
  (return false))

(fn ICheckControled
  (params (A :type Actor%20Object%20Reference))
  (return false 0))

(fn ICheckCurrentAction
  (params (Action :type Action%20Enum :default "NewEnumerator0"))
  (return false))

(fn ICurrentAction
  (return "NewEnumerator0"))

(fn ICurrentLevelDisplayName
  (return ""))

(fn ICurrentTarget
  (return 0 false))

(fn IDetectEnemy
  (params (Max :type Float%20%28single-precision%29) (Min :type Float%20%28single-precision%29) (ByClass :type Actor%20Class%20Reference) (Stat :type EEnemyStat%20Enum :default "NewEnumerator0"))
  (return (Utilities|Array|MakeArray (Variables|Default|GetImpotantEnemy))))

(fn IEmotion
  (return "NewEnumerator0"))

(fn IGetCurrentAction
  (return "NewEnumerator0"))

(fn IGetCurrentGameSave
  (params (reload :type Boolean) (PlayerId :type Integer))
  (return 0 0))

(fn IGetCurrentQuest
  (return "NewEnumerator0"))

(fn IGetLang
  (return "NewEnumerator0"))

(fn IGetLevel
  (return 0))

(fn IGetMissionStat
  (return "NewEnumerator0"))

(fn IGetSignGroup
  (return (Variables|Default|GetSign) (Variables|Default|GetGroupID) (Variables|Default|GetChannel)))

(fn IGetTarget
  (return 0 false))

(fn IgettextBylang
  (params (lang :type Elang%20Enum :default "NewEnumerator0"))
  (return ""))

(fn IisDied
  (return false))

(fn IisNewGame
  (return false))

(fn ILoadProfile
  (params (name :type String))
  (return 0))

(fn ILostTarget
  (return false false))

(fn IMapLevelActived
  (params (MapName :type EMapName%20Enum :default "NewEnumerator0") (InList :type Array%20of%20EMapName%20Enums))
  (return false))

(fn INoAction
  (return false))

(fn IPlayerControled
  (params (actor :type Actor%20Object%20Reference))
  (return false))

(fn IPlayerName
  (return ""))

(fn IreachGoal
  (params (Dist :type Float%20%28single-precision%29))
  (bind _dist (Utilities|MxDirectiontoLocation (Variables|Default|GetMissionLocation)))
  (return (< _dist Dist)))

(fn IRequestLocation
  (return "0, 0, 0"))

(fn ISameSide
  (params (TestActor :type Actor%20Object%20Reference))
  (Utilities|IsValid TestActor
    (:Is%20Valid
      (bind _sign (Class|Human|GetSign(Message) TestActor))
      (return (== (Variables|Default|GetSign) _sign)))
    (:Is%20Not%20Valid
      (return true))))

(fn ISelectAble
  (return false))

(fn IsMapActive
  (params (Map%20name :type EMapName%20Enum :default "NewEnumerator0"))
  (return false))

(fn ITargetRelation
  (params (New%20Target :type Actor%20Object%20Reference) (UseCurrent :type Boolean))
  (return false 0.0 "0, 0, 0" 0.0))

(fn ITracktoActor
  (params (Actor :type Actor%20Object%20Reference) (Dist :type Float%20%28single-precision%29))
  (return false))

(fn ITutorialShow
  (return false))

(fn UpdateAction
  (return "NewEnumerator0" false "0, 0, 0" 0.0))