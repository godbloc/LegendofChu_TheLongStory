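; Camera actor that takes over the player view and orbits a ViewTarget point at a fixed rotation and distance.
; Interface events drive timelines that snap to a location, follow an actor until it dies or is out of range, pan with damped speed, and smooth-zoom.
; UpdateCamPositionByTarget repositions the camera from ViewTarget; smooth zoom also scales screen percentage with distance.
; Extra events add quake shake and a circling fly-around.
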(event `SnapViewToLocation`
  (params (Location :type "Vector Structure"))
  ;[1 1 1] SnapView To Location
  (set `self.PanSpeed` (0.0 0.0 0.0))
  (bind (_direction _newtrack_0) (`Timeline|Timeline_1` :!via `PlayFromStart` :!label _label)
    (:`Update`
      (set `self.ViewTarget` (`KismetMathLibrary.VLerp` (`self.ViewTarget`) Location _newtrack_0))
      (`self.UpdateCamPositionByTarget`))))

(event `StopSnap`
  ;[1 1 1] SnapView To Location
  (goto _label :!via `Stop`))

(event `StopFollow`
  (bind _viewtarget (`self.ViewTarget`))
  ;[1 1 1] Snap view to actor
  (bind (_direction _newtrack_0) (`Timeline|Timeline_0` :!via `Stop` :!label _label_2)
    (:`Update`
      (bind _result (message `/Game/Game/Blueprints/Human.iisDied` (stale `SnapViewToActor` ActorTarget)))
      (if _result
        (`self.StopFollow` :!label _label_3)
        (else
          (bind (_direction_2 _dist) (`/Game/common/GXFuncs_v9.xDirectionToActor` (stale `SnapViewToActor` ActorTarget) _viewtarget))
          (if (< _dist 9999.0)
            (bind _returnvalue (`KismetMathLibrary.VLerp` _direction_2 (0.0 0.0 0.0) _newtrack_0))
            (bind _output_get (set `self.ViewTarget` (+ _viewtarget _returnvalue)))
            (if (stale `SnapViewToActor` KeepRotation)
              (`self.K2_AddActorWorldOffset` _returnvalue true)
              (else
                (`/Game/NewChuAccess/Bp/MX_LibA.Mx_LookAtLocationOrActor` (stale `SnapViewToActor` _output_get) _output_get)))
            (else
              (goto _label_3))))))))

(event `/Game/Game/Blueprints/iGAME.iSnapViewtoTarget`
  (params (Target :type "Actor Object Reference") (KeepRotation :type Boolean))
  ;[1 1 1] GameInterface
  ;;[1 1 1] SnapView To Targert
  (`self.SnapViewToActor` KeepRotation Target true))

(event `SnapViewToActor`
  (params (KeepRotation :type Boolean) (ActorTarget :type "Actor Object Reference") (`Keep Distance` :type Boolean))
  ;[1 1 1] Snap view to actor
  (`/Engine/EditorBlueprintResources/StandardMacros.IsValid` ActorTarget
    (:`Is Valid`
      (bind _output_get (set `self.Target` ActorTarget))
      (goto _label_2 :!via `PlayFromStart`))))

(event `/Game/Game/Blueprints/iCamera.iSnapViewToLocation`
  (params (Location :type "Vector Structure"))
  ;[1 1 1] GameInterface
  ;;[1 1 1] SnapView To Targert
  (`self.SnapViewToLocation` Location))

(event `ResetAspect`
  (bind (_x _y) (`KismetMathLibrary.BreakVector2D` (`WidgetLayoutLibrary.GetViewportSize`)))
  ;[1 1 1] Reset Aspect
  (set `CameraComponent.AspectRatio` (/ _x _y) (`self.CameraComponent`)))

(event `self.ReceiveBeginPlay`
  ;[1 1 1] Begin And Tick
  (`KismetSystemLibrary.Delay` 0.1)
  (`self.ResetAspect`)
  (`self.ActiveView` 1.0))

(event `UpdatePosition`
  ;[1 1 1] Update position
  (if (`self.Free`)
    (`self.LookAtActor` (`self.K2_GetActorLocation` (`self.Target`)))
    (elif (`self.Dynamic`)
      (`self.MovingCam_TransForm`)
      (else
        (`self.MovingCam`)))))

(event `ActiveView`
  (params (`blend time` :type "Float (double-precision)"))
  ;[1 1 1] ActiveView
  (`PlayerController.SetViewTargetWithBlend` (`GameplayStatics.GetPlayerController` 0) self `blend time` "VTBlend_Linear" 0.0 false)
  (`self.ResetAspect`))

(event `ActiveToTarget`
  (params (Target :type "Actor Object Reference") (BlendTime :type "Float (double-precision)"))
  ;[1 1 1] Active With Actor
  (set `self.Target` Target)
  (`PlayerController.SetViewTargetWithBlend` (`GameplayStatics.GetPlayerController` 0) self BlendTime "VTBlend_Linear" 0.0 false)
  (`self.ResetAspect`))

(event `Playquake`
  ;[1 1 1] PlayQuake
  (`self.DQuakeActive`)
  (bind (_direction _quake) (`Timeline|QuakeTime` :`NewTime` 0.01 :!via `PlayFromStart`)
    (:`Update`
      (`self.K2_SetActorLocation` (+ (* _quake 100.0) (`self.K2_GetActorLocation`))))
    (:`Finished`
      (`self.DQuakeEnd`))))

(event `CamPlayAround`
  (params (`time deli` :type "Float (double-precision)"))
  (bind _returnvalue (`self.K2_GetActorLocation`))
  (bind _targetlength (`self.targetLength`))
  ;[1 1 1] PlayAround
  (set `self.Free` true)
  (bind _output_get (set `self.targetLocation` (+ (* (`KismetMathLibrary.Normal` (`self.GetActorForwardVector`)) (`self.targetLength`)) _returnvalue)))
  (bind (_direction _movearound) (`Timeline|PlayAround` :`NewTime` 0.0 :!via `PlayFromStart`)
    (:`Update`
      (bind _returnvalue_2 (* _movearound 360.0))
      (`self.K2_SetActorLocation` (+ (`KismetMathLibrary.MakeVector` (* _targetlength (`KismetMathLibrary.DegSin` _returnvalue_2)) (* (`KismetMathLibrary.DegCos` _returnvalue_2) _targetlength) 0.0) _output_get) true)
      (`self.K2_SetActorRotation` (`KismetMathLibrary.FindLookAtRotation` _returnvalue _output_get)))
    (:`Finished`
      (set `self.Free` false))))

(event `/Game/Game/Blueprints/iCamera.iZoom`
  (params (Delta :type "Float (single-precision)") (isFovOrLoc :type Boolean))
  (bind _cameracomponent (`self.CameraComponent`))
  ;[1 1 1] Zoom
  (if true
    (set `CameraComponent.FieldOfView` (`KismetMathLibrary.FClamp` (+ (`CameraComponent.FieldOfView` _cameracomponent) Delta) 30.0 120.0) _cameracomponent)
    (else
      (`self.K2_AddActorWorldOffset` (* (`self.GetActorForwardVector`) Delta)))))

(event `/Game/Game/Blueprints/iCamera.iSmoothZoom`
  (params (NewDist :type "Float (single-precision)") (isSet :type Boolean))
  ;[1 1 1] ZoomIn
  (if isSet
    (`self.SmoothZoom` (`KismetMathLibrary.FClamp` NewDist 500.0 9000.0))
    (else
      (`self.SmoothZoom` (`KismetMathLibrary.FClamp` (+ (`self.MaxDistance`) NewDist) 500.0 9000.0)))))

(event `SmoothZoom`
  (params (`New Dist` :type "Float (double-precision)"))
  ;[1 1 1] ZoomIn
  (`Timeline|ZoomByDist` :!via `PlayFromStart`
    (:`Update`
      (bind _output_get (set `self.MaxDistance` (`KismetMathLibrary.Lerp` (`self.MaxDistance`) `New Dist` 0.5)))
      (`self.UpdateCamPositionByTarget`)
      (setmembers `PostProcessSettings` :`StructRef` (`CameraComponent.PostProcessSettings` (`self.CameraComponent`)) :`ScreenPercentage` (`KismetMathLibrary.FClamp` (* (/ (- 10000.0 _output_get) 10000.0) 100.0) 30.0 200.0)))
    (:`Finished`
      (set `self.MaxDistance` `New Dist`)
      (`self.UpdateCamPositionByTarget`))))

(event `/Game/Game/Blueprints/iCamera.iCameraRestore`
  (params (Zoom :type Boolean))
  ;[1 1 1] ZoomIn
  (if Zoom
    (`self.SmoothZoom` (`self.PreviewDist`))))

(event `/Game/Game/Blueprints/iCamera.iPanning`
  (params (Offset :type "Vector Structure"))
  (bind _panspeed (`self.PanSpeed`))
  ;[1 1 1] Panning
  (bind _returnvalue (`self.2dVectorTo3d` Offset))
  (set `self.PanSpeed` (+ (`self.PanSpeed`) _returnvalue))
  (`Timeline|Panning` :!label _label_4
    (:`Update`
      (set `self.ViewTarget` (+ (`self.ViewTarget`) _panspeed))
      (`self.UpdateCamPositionByTarget`)
      (set `self.PanSpeed` (`KismetMathLibrary.VLerp` _panspeed (0.0 0.0 0.0) 0.1)))))

(event `StopPanning`
  ;[1 1 1] Panning
  (goto _label_4 :!via `Stop`))

(fn `2dVectorTo3d`
  (params (InVec :type "Vector Structure"))
  (returns (ReturnValue :type "Vector Structure"))
  (return (+ (* (`self.GetActorRightVector`) (* (.x InVec) -1.0)) (* (`KismetMathLibrary.Normal` (* (`self.GetActorForwardVector`) (1.0 1.0 0.0))) (.y InVec)))))

(fn `iCurrentLevelDisplayName`
  (returns (name :type String))
  (return ""))

(fn `iGetCurrentQuest`
  (returns (QuestName :type "/Game/Game/Blueprints/QuestData/EQuestName Enum"))
  (return "NewEnumerator0"))

(fn `iGetLang`
  (returns (result :type "/Game/Game/Blueprints/Cdt_lang Enum"))
  (return "NewEnumerator0"))

(fn `igettextBylang`
  (params (lang :type "/Game/Game/Blueprints/Elang Enum" :default "NewEnumerator0"))
  (returns (result :type String))
  (return ""))

(fn `iisNewGame`
  (returns (value :type Boolean))
  (return false))

(fn `iLoadProfile`
  (params (name :type String))
  (returns (save :type "/Game/Game/Blueprints/CDTSave Object Reference"))
  (return null))

(fn `iMapLevelActived`
  (params (MapName :type "/Game/Game/Enums/EMapName Enum" :default "NewEnumerator0") (InList :type "Array of /Game/Game/Enums/EMapName Enum (by ref)"))
  (returns (Actived :type Boolean))
  (return false))

(fn `iPlayerName`
  (returns (`Player name` :type String))
  (return ""))

(fn `IsMapActive`
  (params (`Map name` :type "/Game/Game/Enums/EMapName Enum" :default "NewEnumerator0"))
  (returns (result :type Boolean))
  (return false))

(fn `iTutorialShow`
  (returns (Result :type Boolean))
  (return false))

(fn `UpdateCamPositionByTarget`
  (`self.K2_SetActorLocation` (- (`self.ViewTarget`) (* (`KismetMathLibrary.GetForwardVector` (`self.InitialRotation`)) (`self.MaxDistance`)))))

(fn `UserConstructionScript`
  (bind _target (`self.Target`))
  (bind _previewdist (`self.PreviewDist`))
  (`self.RefreshTargetDistance`)
  (if (`self.Lock`)
    (`self.K2_SetActorRotation` (`self.InitialRotation`))
    (`self.SmoothZoom` _previewdist)
    (set `self.MaxDistance` _previewdist)
    (else
      (set `self.InitialRotation` (`self.K2_GetActorRotation`))
      (`/Engine/EditorBlueprintResources/StandardMacros.IsValid` _target
        (:`Is Valid`
          (`self.SnapViewToActor` true _target true))))))