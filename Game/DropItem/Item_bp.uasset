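; Pickup item actor that takes its data and billboard icon from Tb_ItemData, using its type enum as row index in construction.
; It spawns with an upward velocity and particle burst, and shows its name widget while the player is in the Affect volume.
; Sphere overlap (if active) or IGainItem reports it to the player and fires a picked call.
; Looping items hide, then reappear after a delay; others are destroyed with a burst.
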(event `self.ReceiveDestroyed`
  ;[1 1 1] Destroy
  (`GameplayStatics.SpawnEmitterAtLocation` "/Game/InfinityBladeEffects/Effects/FX_Combat_Base/WeaponCombo/P_ComboFinish_Tap_02.P_ComboFinish_Tap_02" (`self.K2_GetActorLocation`)))

(event `/Game/Game/DropItem/iItem.iGainItem`
  (params (Actor :type "Actor Object Reference"))
  ;[1 1 1] GainItem
  (`self.DoGainItem` Actor))

(event `DoGainItem`
  (params (Actor :type "Actor Object Reference"))
  ;[1 1 1] GainItem
  (if (not (`self.bHidden`))
    (bind _result (`/Game/common/GXFuncs_v9.isControlPlayer` Actor))
    (if _result
      (message `/Game/Game/Interface/iQuest.iTemReport` Actor self)
      (if (`self.CanLoop`)
        (`self.SetActorHiddenInGame` true)
        (`KismetSystemLibrary.Delay` (`self.timedelay`))
        (`self.SetActorHiddenInGame` false)
        (`self.DPicked`)
        (else
          (`KismetSystemLibrary.Delay` 0.2)
          (`self.K2_DestroyActor`))))))

(event `self.Sphere.OnComponentBeginOverlap`
  (params (OverlappedComponent :type "PrimitiveComponent Object Reference") (OtherActor :type "Actor Object Reference") (OtherComp :type "PrimitiveComponent Object Reference") (OtherBodyIndex :type Integer) (bFromSweep :type Boolean) (SweepResult :type "HitResult Structure (by ref)"))
  ;[1 1 1] GainItem
  (if (`self.Actived`)
    (`self.DoGainItem` OtherActor)
    (`GameplayStatics.PlaySound2D` "/Game/Sound/Bell_drum__high_Cue.Bell_drum__high_Cue")))

(event `MakeItem`
  (params (Type :type "/Game/Game/DropItem/EitemName Enum"))
  ;[1 1 1] Gern Item
  (bind _item (`self.GetItemByIndex` (`KismetMathLibrary.Conv_ByteToInt` (`KismetSystemLibrary.MakeLiteralByte` Type))))
  (set `self.data` _item)
  (`BillboardComponent.SetSprite` (`self.Billboard`) (`.Icon_38_9097B5B84EE4D148F956B1906188730E` (break `/Game/Game/DropItem/Item_Struct` _item))))

(event `self.ReceiveBeginPlay`
  ;[1 1 1] Gern Item
  (`GameplayStatics.SpawnEmitterAtLocation` "/Game/InfinityBladeEffects/Effects/FX_Combat_Base/WeaponCombo/P_ComboFinish_Tap_02.P_ComboFinish_Tap_02" (`self.K2_GetActorLocation`))
  (set `MovementComponent.Velocity` (0.0 0.0 100.0) (`self.ProjectileMovement`)))

(event `self.Affect.OnComponentBeginOverlap`
  (params (OverlappedComponent :type "PrimitiveComponent Object Reference") (OtherActor :type "Actor Object Reference") (OtherComp :type "PrimitiveComponent Object Reference") (OtherBodyIndex :type Integer) (bFromSweep :type Boolean) (SweepResult :type "HitResult Structure (by ref)"))
  ;[1 1 1] Play animation
  (bind _result (`/Game/common/GXFuncs_v9.isControlPlayer` OtherActor))
  (if _result
    (`self.DoShowItem`)))

(event `self.Affect.OnComponentEndOverlap`
  (params (OverlappedComponent :type "PrimitiveComponent Object Reference") (OtherActor :type "Actor Object Reference") (OtherComp :type "PrimitiveComponent Object Reference") (OtherBodyIndex :type Integer))
  ;[1 1 1] Play animation
  (bind _result (`/Game/common/GXFuncs_v9.isControlPlayer` OtherActor))
  (if _result
    (`SceneComponent.SetHiddenInGame` (`self.Widget`) true false)))

(event `DoShowItem`
  (bind _widget (`self.Widget`))
  ;[1 1 1] Play animation
  (`SceneComponent.SetHiddenInGame` _widget false false)
  (message `/Game/MenuWidget/iWidget.iShowText` (`WidgetComponent.GetUserWidgetObject` _widget) (`.EnName_14_E3C904BD4E035AB277BAE696E1358B3C` (break `/Game/Game/DropItem/Item_Struct` (`self.data`))) ""))

(fn `getItemByEname`
  (params (Ename :type "/Game/Game/DropItem/EitemName Enum"))
  (returns (item :type "/Game/Game/DropItem/Item_Struct Structure") (ReturnValue :type Boolean))
  (bind _outrownames (`DataTableFunctionLibrary.GetDataTableRowNames` "/Game/Game/DropItem/Tb_ItemData.Tb_ItemData"))
  (for _array_element _outrownames
    (bind _returnvalue (`|GetDataTableRow` "/Game/Game/DropItem/Tb_ItemData.Tb_ItemData" _array_element)
      (:`then`
        (bind _returnvalue_2 (`|EnumEquality` Ename (`.TypeName_3_8A8EB605405F0743DAA45ABE79CC677C` (break `/Game/Game/DropItem/Item_Struct` _returnvalue))))
        (if _returnvalue_2
          (set `self.data` _returnvalue)
          (break)))))
  (return (`self.data`) _returnvalue_2))

(fn `GetItemByIndex`
  (params (Index :type Integer))
  (returns (item :type "/Game/Game/DropItem/Item_Struct Structure"))
  (bind _outrownames (`DataTableFunctionLibrary.GetDataTableRowNames` "/Game/Game/DropItem/Tb_ItemData.Tb_ItemData"))
  (bind _returnvalue (`|GetDataTableRow` "/Game/Game/DropItem/Tb_ItemData.Tb_ItemData" (`KismetArrayLibrary.Array_Get` _outrownames Index))
    (:`then`
      (set `self.data` _returnvalue))
    (:`RowNotFound`
      _))
  (return (`self.data`)))

(fn `UserConstructionScript`
  (`self.MakeItem` (`self.ename`)))