(event OnComponentBeginOverlap(EffectRegione)
  (params (OverlappedComponent :type Primitive%20Component%20Object%20Reference) (OtherActor :type Actor%20Object%20Reference) (OtherComp :type Primitive%20Component%20Object%20Reference) (OtherBodyIndex :type Integer) (bFromSweep :type Boolean) (SweepResult :type Hit%20Result%20Structure%20%28by%20ref%29))
  (Utilities|FlowControl|Gate true
    (:Exit
      (Class|CdtSkill|EnableEffect(Message) OtherActor (Variables|Default|GetAbsoreEffect)))))

(event Custom|DGetAngry_Event
  (Utilities|FlowControl|Gate true) ; enters at Open
)

(event Custom|Disapear
  (params (Active :type Boolean))
  (bind _mesh (Variables|Character|GetMesh))
  (bind _returnvalue (Components|SkeletalMesh|GetAnimInstance _mesh))
  (Variables|Default|SetSleepy Active)
  (Variables|Default|SetbCanBeDamaged (not Active))
  (if Active
    (Class|IMonster|IUnSummon(Message) _returnvalue)
    (else
      (Class|IMonster|ISummoned(Message) _returnvalue))))

(event Custom|EnableEffect
  (params (Effector :type Actor%20Object%20Reference))
  (Variables|Default|SetAbsoreEffect (stale Custom|CastEffect effector)))

(event Custom|CastEffect
  (params (effector :type Actor%20Object%20Reference) (lifetime :type Float%20%28single-precision%29 :default 0.0))
  (Variables|Default|SetAbsoreEffect (stale Custom|EnableEffect Effector)))

(event Custom|iCastSkill
  (params (SkillType :type Integer :default 0) (SkillName :type ESkillName%20Enum :default "NewEnumerator0"))
  (Utilities|FlowControl|Gate true) ; enters at Open
)

(event Custom|doBegin
  (Transformation|SetRelativeLocation (Variables|Character|GetMesh) "0, 0,-90.000000" false false))

(event EventBeginPlay
  (CallFunction|Disapear (Variables|Default|GetSleepy))
  (bind _returnvalue (UserInterface|CreateWidget "/Game/MenuWidget/Wg_SummonTimeBar.Wg_SummonTimeBar_C" 0 self))
  (UserInterface|SetWidget (Variables|Default|GetWgSummonBar) _returnvalue))

(event EventTick
  (params (DeltaSeconds :type Float%20%28single-precision%29))
  (Utilities|FlowControl|Delay 0.2)
  (CallFunction|DoSummonTime DeltaSeconds)
  (Utilities|MSummonStat
    (:Can%20Summon
      (if (Variables|Auto|GetAutoSummon)
        (CallFunction|Disapear false)))
    (:Unsummon
      (CallFunction|Disapear true))))

(event EventISummoned
  (params (Owner :type Actor%20Object%20Reference) (GfType :type Integer) (Sign :type Integer))
  (Variables|Default|SetSummoner Owner))

(fn ConstructionScript
  (|CallParentFunction)
  (Development|SetHiddeninGame (Variables|Default|GetPa_Aura_Water) (Variables|Default|GetSleepy) false))

(fn FadeinScale
  (params (Delegate :type Delegate))
  (bind _rockass (Variables|Default|GetRockAss))
  (bind _returnvalue (Transformation|GetActorScale3D _rockass))
  (Transformation|SetActorScale3D _rockass (* _returnvalue 0.95))
  (if (< (Math|Vector|VectorLength _returnvalue) 0.1)
    (Class|KismetSystemLibrary|ClearTimerHandle)
    (Actor|DestroyActor _rockass))
  (return))

(fn DoSummonTime
  (params (Rate :type Float%20%28single-precision%29))
  (if (Variables|Default|GetSleepy)
    (Variables|Default|SetSummonTimeRemain_0 (Math|Float|Clamp(Float) (+ (Variables|Default|GetSummonTimeRemain_0) Rate)))
    (else
      (Variables|Default|SetSummonTimeRemain_0 (Math|Float|Clamp(Float) (- (Variables|Default|GetSummonTimeRemain_0) Rate)))))
  (return (Variables|Default|GetSummonTimeRemain_0)))

(fn IGetSummonTimeRemain
  (return (Variables|Default|GetSummonTimeRemain_0)))

(fn ISelectAble
  (return false))

(fn IGetSignGroup
  (return 0 0 0))

(fn ITargetRelation
  (params (New%20Target :type Actor%20Object%20Reference) (UseCurrent :type Boolean))
  (return false 0.0 "0, 0, 0" 0.0))

(fn IGetCurrentAction
  (return "NewEnumerator0"))

(fn ICheckCurrentAction
  (params (Action :type Action%20Enum :default "NewEnumerator0"))
  (return false))

(fn ICurrentAction
  (return "NewEnumerator0"))

(fn INoAction
  (return false))

(fn IBusy
  (return false false))

(fn ICannotFocus
  (return false))

(fn IGetLevel
  (return 0))

(fn GetSign
  (return 0))

(fn IPlayerControled
  (params (actor :type Actor%20Object%20Reference))
  (return false))

(fn ISameSide
  (params (TestActor :type Actor%20Object%20Reference))
  (return false))

(fn IEmotion
  (return "NewEnumerator0"))

(fn IRequestLocation
  (return "0, 0, 0"))

(fn IisDied
  (return false))

(fn GetAttkInfo
  (return false 0 0 "NewEnumerator0"))

(fn GetCritChance
  (return 0.0))

(fn UpdateAction
  (return "NewEnumerator0" false "0, 0, 0" 0.0))

(fn CharaterProperties
  (return 0.0 false false))