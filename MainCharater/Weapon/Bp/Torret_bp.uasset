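; Stationary turret that fires skill projectiles at characters not on its side within a radius set at construction.
; While active, Tick uses a random Delay, then shoots a random Bullet class at each hostile overlap; skills added by name extend that list.
; Damage accumulates, awarding attackers XP, until exceeding HP triggers delayed destruction.
; Character interface functions mostly return inert defaults, with side identity read from CPBase.
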(event Custom|Bedestroyed
  (params (Causer :type Actor%20Object%20Reference))
  (Utilities|FlowControl|Delay 1.0)
  (Actor|DestroyActor))

(event Game|Damage|EventAnyDamage
  (params (Damage :type Float%20%28single-precision%29) (DamageType :type Damage%20Type%20Object%20Reference) (InstigatedBy :type Controller%20Object%20Reference) (DamageCauser :type Actor%20Object%20Reference))
  (Utilities|IsValid DamageCauser
    (:Is%20Valid
      (bind _output_get (Variables|Default|SetDamaged (+ (Variables|Default|GetDamaged) Damage)))
      (Effects|SpawnEmitteratLocation "/Game/ParticleSystem/PaticularEffect/Effects/Aura/growup_Fire.growup_Fire" (Transformation|GetActorLocation))
      (if (> _output_get (Variables|Default|GetHP))
        (Default|CallDbeDestroyed DamageCauser)
        (Class|Human|IXPUp(Message) DamageCauser 50)
        (CallFunction|Bedestroyed DamageCauser)
        (else
          (Class|Human|IXPUp(Message) DamageCauser 1))))))

(event EventTick
  (params (DeltaSeconds :type Float%20%28single-precision%29))
  (bind _bullet (Variables|Default|GetBullet))
  (if (Variables|Default|GetActived)
    (Utilities|FlowControl|Delay (Math|Random|RandomFloatinRange 0.5 2.0))
    (for _array_element (Collision|GetOverlappingActors (Variables|Default|GetSphere) "/Game/NewChuAccess/Bp/Cdt_Dummy_New.Cdt_Dummy_New_C" :!class /Script/Engine.PrimitiveComponent)
      (bind _result (Class|Human|ISameSide(Message) _array_element self))
      (if (not _result)
        (bind _direction (Utilities|MxDirection _array_element true false))
        (CallFunction|Projectile (Utilities|Array|Get(acopy) _bullet (Math|Random|RandomInteger (Utilities|Array|Length _bullet))) 1e+02 111.0 111.0 self (Transformation|GetWorldLocation (Variables|Default|GetArrow)) _direction _array_element true "1.000000,1.000000,1.000000")))))

(event EventIAddSkilltoSkillList
  (params (SkillName :type ESkillName%20Enum :default "NewEnumerator0") (Remove :type Boolean))
  (bind _out_row (CallFunction|XSkillbyEname SkillName))
  (Utilities|Array|Add (Variables|Default|GetBullet) (.SkillClass (Utilities|Struct|BreakSkillStruct _out_row))))

(fn ConstructionScript
  (Components|Sphere|SetSphereRadius (Variables|Default|GetSphere) (Variables|Default|GetRadius) true))

(fn CharaterProperties
  (return 0.0 false false))

(fn GetAttkInfo
  (return false 0 0 "NewEnumerator0"))

(fn GetCritChance
  (return 0.0))

(fn GetSign
  (return (Variables|/Game/Game/Blueprints/CP_Base.CP_Base_C|GetSign (Variables|Default|GetCP_Base))))

(fn IBusy
  (return false false))

(fn ICanCastSkill
  (return false false "NewEnumerator0"))

(fn ICannotFocus
  (return false))

(fn ICheckCurrentAction
  (params (Action :type Action%20Enum :default "NewEnumerator0"))
  (return true))

(fn ICurrentAction
  (return "NewEnumerator0"))

(fn IEmotion
  (return "NewEnumerator0"))

(fn IGetCurrentAction
  (return "NewEnumerator0"))

(fn IGetLevel
  (return 0))

(fn IGetSignGroup
  (bind _cp_base (Variables|Default|GetCP_Base))
  (return (Variables|/Game/Game/Blueprints/CP_Base.CP_Base_C|GetSign _cp_base) (Variables|/Game/Game/Blueprints/CP_Base.CP_Base_C|GetGroup _cp_base) (Variables|/Game/Game/Blueprints/CP_Base.CP_Base_C|GetChannel _cp_base)))

(fn IisDied
  (return false))

(fn INoAction
  (return false))

(fn IPlayerControled
  (params (actor :type Actor%20Object%20Reference))
  (return false))

(fn IRequestLocation
  (return "0, 0, 0"))

(fn ISameSide
  (params (TestActor :type Actor%20Object%20Reference))
  (Utilities|IsValid TestActor
    (:Is%20Valid
      (bind _sign (Class|Human|GetSign(Message) TestActor))
      (return (== _sign (Variables|/Game/Game/Blueprints/CP_Base.CP_Base_C|GetSign (Variables|Default|GetCP_Base)))))
    (:Is%20Not%20Valid
      (return true))))

(fn ISelectAble
  (return false))

(fn ITargetRelation
  (params (New%20Target :type Actor%20Object%20Reference) (UseCurrent :type Boolean))
  (return false 0.0 "0, 0, 0" 0.0))

(fn UpdateAction
  (return "NewEnumerator0" false "0, 0, 0" 0.0))