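; Dragon head homing projectile that launches with an upward kick, scales up on a timeline and chases its target.
; BeginPlay picks one of three steering methods, which Tick runs with a random chance to bend velocity toward the target at differing clamped speeds.
; Hitting an enemy Human, stopping or taking damage triggers Destruc2 for direct plus falloff radial damage and destroys the actor.
; Destruc1 and Destruc3 are unused alternative impact behaviours.
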(event `self.ReceiveDestroyed`
  (bind _returnvalue (`self.K2_GetActorLocation`))
  ;[1 1 1] Destroy Actor
  (`GameplayStatics.PlaySoundAtLocation` (`self.soundfx`) _returnvalue)
  (`GameplayStatics.SpawnEmitterAtLocation` (`self.pp2`) _returnvalue))

(event `SelfDestructive`
  ;[1 1 1] Destructive
  (`self.Destruc2` :!label _label)
  (`self.K2_DestroyActor`))

(event `self.ProjectileMovement_0.OnProjectileStop`
  (params (ImpactResult :type "HitResult Structure (by ref)"))
  ;[1 1 1] Destructive
  (goto _label))

(event `/Game/MainCharater/Weapon/Setting/ThrowWeapon.projectile`
  (params (Direction :type "Vector Structure") (speed :type "Float (single-precision)") (control :type "Float (single-precision)") (Luncher :type "Actor Object Reference") (`can hook` :type Boolean) (target :type "Actor Object Reference") (BaseDamage :type "Float (single-precision)") (AffectR :type "Float (single-precision)"))
  ;[1 1 1] Projective
  (set `MovementComponent.Velocity` (+ (* Direction speed) (0.0 0.0 2000.0)) (`self.ProjectileMovement_0`))
  (set `self.SnapActor` target)
  (set `self.luncher` Luncher)
  (set `self.can Hook` `can hook`)
  (set `self.control` control)
  (set `self.speed` speed)
  (set `self.pDamage` BaseDamage)
  (set `self.radius` AffectR)
  (bind (_direction _newtrack_0) (`Timeline|Timeline_0` :!via `PlayFromStart`)
    (:`Update`
      (`self.SetActorScale3D` (`KismetMathLibrary.Conv_DoubleToVector` _newtrack_0)))
    (:`Finished`
      (`self.SetActorEnableCollision` true :!label _label_2))
    (:`NewTrack_1`
      (`/Engine/EditorBlueprintResources/StandardMacros.FlipFlop`
        (:`A`
          (goto _label_2))
        (:`B`
          (`self.SetActorEnableCollision` false))))))

(event `self.ReceiveTick`
  (params (DeltaSeconds :type "Float (single-precision)"))
  ;[1 1 1] HOOKING
  (`/Engine/EditorBlueprintResources/StandardMacros.IsValid` (`self.SnapActor`)
    (:`Is Valid`
      (switch `int` (`self.Type`)
        (:`Default`
          (`self.MeThod3` :!label _label_3))
        (:`0`
          (`self.MeThod1`))
        (:`1`
          (`self.MeThod2`))
        (:`2`
          (goto _label_3))))))

(event `self.ReceiveBeginPlay`
  ;[1 1 1] HOOKING
  (set `self.Type` (`KismetMathLibrary.RandomIntegerInRange` 0 2)))

(event `self.Bound.OnComponentHit`
  (params (HitComponent :type "PrimitiveComponent Object Reference") (OtherActor :type "Actor Object Reference") (OtherComp :type "PrimitiveComponent Object Reference") (NormalImpulse :type "Vector Structure") (Hit :type "HitResult Structure (by ref)"))
  ;[1 1 1] OVVERLAP
  (if (`KismetSystemLibrary.DoesImplementInterface` OtherActor "/Game/Game/Blueprints/Human.Human_C")
    (bind _result (message `/Game/Game/Blueprints/Human.iSameSide` OtherActor (`self.luncher`)))
    (if (not _result)
      (set `self.SnapActor` OtherActor)
      (`self.SelfDestructive`))))

(fn `TakeDamage`
  (returns (Damage :type "Float (double-precision)"))
  (`self.SelfDestructive`)
  (return (`self.pDamage`)))

(fn `UserConstructionScript`
  (`self.SetActorEnableCollision` false))