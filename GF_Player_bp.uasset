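; Summoned GF companion character that fights for its Summoner, taking mesh, anim class and movement mode from a data table by type.
; AI controller and blackboard drive missions and targets, while Tick steers toward the mission location and refreshes a summoner beam, recalling it when distant.
; Attacks apply skill-table damage, blasts and projectiles scaled by Rank.
; Hostile damage drains summon time until it unsummons, hiding and disabling rather than destroying the actor.
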(event `self.ReceiveBeginPlay`
  (if (`self.AutoSummon`)
    (`self.iSummoned` (`self.Summoner`) (`self.Gdtype`) (`self.GfSign`))))

(event `self.ReceiveTick`
  (params (DeltaSeconds :type "Float (single-precision)"))
  (bind _location (`self.Location`))
  (`|ExecutionSequence`
    (:`then_0`
      (`KismetSystemLibrary.Delay` 3.0)
      (`self.LinkToSummoner`))
    (:`then_1`
      (if (== _location (0.0 0.0 0.0))
        (set `self.Location` (`self.K2_GetActorLocation`))
        (else
          (bind (_success _returnvalue) (`self.GetSteeringValue` _location))
          (`self.iSteering` _returnvalue))))))

(event `/Game/Game/Blueprints/Human.iChooseTypeAndSign`
  (params (`Actor Type` :type Integer) (sign :type Integer))
  (bind _mesh (`self.Mesh`))
  (bind _charactermovement (`self.CharacterMovement`))
  (set `self.Gdtype` `Actor Type`)
  (bind _outrownames (`DataTableFunctionLibrary.GetDataTableRowNames` "/Game/NewChuAccess/Monster_Character/Gf_Table.Gf_Table"))
  (bind _returnvalue (`|GetDataTableRow` "/Game/NewChuAccess/Monster_Character/Gf_Table.Gf_Table" (`KismetArrayLibrary.Array_Get` _outrownames `Actor Type`))
    (:`then`
      (bind (_class _skmesh _animclass) (break `/Game/NewChuAccess/Monster_Character/GF_Struct` _returnvalue))
      (`SkinnedMeshComponent.SetSkinnedAssetAndUpdate` _mesh _skmesh true)
      (`SkeletalMeshComponent.SetAnimInstanceClass` _mesh _animclass)
      (set `/Game/Game/Blueprints/CP_Base.Sign` sign (`self.CP_Base`))
      (switch `int` `Actor Type`
        (:`0`
          (set `CharacterMovementComponent.MaxWalkSpeed` 1500.0 _charactermovement :!label _label))
        (:`1`
          (`CharacterMovementComponent.SetMovementMode` _charactermovement "MOVE_Flying" 0 :!label _label_2)
          (goto _label))
        (:`2`
          (`CharacterMovementComponent.SetMovementMode` _charactermovement "MOVE_Walking" 0)
          (set `CharacterMovementComponent.MaxWalkSpeed` 1000.0 _charactermovement))
        (:`3`
          (goto _label_2))))))

(event `/Game/Recycle/BossMonster/iMonster.iSummoned`
  (params (Owner :type "Actor Object Reference") (GfType :type Integer) (Sign :type Integer))
  (`self.CreateBBValue`)
  (`/Engine/EditorBlueprintResources/StandardMacros.IsValid` Owner
    (:`Is Valid`
      (bind _output_get (set `self.Summoner` Owner))
      (bind _sign (message `/Game/Game/Blueprints/Human.getSign` _output_get))
      (set `self.GfSign` _sign))
    (:`Is Not Valid`
      (set `self.GfSign` Sign)))
  (`self.iChooseTypeAndSign` GfType (`self.GfSign`))
  (message `/Game/Recycle/BossMonster/iMonster.iSummoned` (`SkeletalMeshComponent.GetAnimInstance` (`self.Mesh`)) Owner GfType Sign)
  (`self.UpdateBlackBoard`)
  (`self.SummonDisapear` true)
  (bind _returnvalue (`|CreateWidget` "/Game/MenuWidget/Wg_SummonTimeBar.Wg_SummonTimeBar_C" null self))
  (`WidgetComponent.SetWidget` (`self.WgTimeRemain`) _returnvalue))

(event `/Game/Recycle/BossMonster/iMonster.iUnSummon`
  (message `/Game/Recycle/BossMonster/iMonster.iUnSummon` (`SkeletalMeshComponent.GetAnimInstance` (`self.Mesh`)))
  (`KismetSystemLibrary.Delay` 3.0)
  (`self.SummonDisapear` false))

(event `/Game/Recycle/BossMonster/iMonster.iSetSummonAction`
  (params (Atk :type Integer) (Speed :type "Float (single-precision)") (Velocity :type "Vector Structure") (Scale :type "Float (single-precision)"))
  (message `/Game/Recycle/BossMonster/iMonster.iSetSummonAction` (`SkeletalMeshComponent.GetAnimInstance` (`self.Mesh`)) Atk Speed Velocity Scale))

(event `/Game/Game/Blueprints/iAnimation.iSteering`
  (params (Steering :type "Float (single-precision)"))
  (bind _returnvalue (`SkeletalMeshComponent.GetAnimInstance` (`self.Mesh`)))
  (`self.K2_AddActorWorldRotation` (`KismetMathLibrary.MakeRotator` 0.0 0.0 (* (* Steering 15.0) 0.1)))
  (message `/Game/Game/Blueprints/iAnimation.iSteering` _returnvalue (* Steering 0.75))
  (message `/Game/Game/Blueprints/iAnimation.iLookAtTarget` _returnvalue (`self.Location`)))

(event `/Game/Game/Blueprints/Human.iMovetoLocation`
  (params (Location :type "Vector Structure") (Limit :type "Float (single-precision)") (rapit :type Boolean) (FaceTo :type Boolean))
  (if (`self.MoveAble`)
    (bind _newparam (`self.ireachGoal` Limit))
    (if _newparam
      (`self.iSetSummonAction` 0 0.0 (0.0 0.0 0.0) (`self.Rank`))
      (else
        (bind (_success _returnvalue) (`self.GetSteeringValue` Location))
        (if (`KismetMathLibrary.NearlyEqual_FloatFloat` _returnvalue 0.0 0.3)
          (`NavigationSystem.SimpleMoveToLocation` (`self.GetController`) Location)
          (bind _direction (`/Game/common/GXFuncs_v9.xDirection` (`self.Location`) Location))
          (`self.AddMovementInput` _direction)
          (`self.iSetSummonAction` 4 1.0 (`self.GetVelocity`) (`self.Rank`)))))))

(event `/Game/Game/Blueprints/iAI.iAISetMission`
  (params (Loc :type "Vector Structure") (Stat :type "/Game/Game/AITree/EMissionStatus Enum" :default "NewEnumerator0"))
  (bind _returnvalue (`AIBlueprintHelperLibrary.GetAIController` self))
  (message `/Game/Game/Blueprints/iAI.iAISetMission` _returnvalue Loc Stat)
  (set `self.Location` Loc))

(event `/Game/Game/Blueprints/iAI.iActiveNewAi`
  (params (`Ai Class` :type "AIController Class Reference") (`Ai Tree` :type "BehaviorTree Object Reference") (`Ai Tb` :type "BlackboardData Object Reference"))
  (bind _returnvalue (`AIBlueprintHelperLibrary.GetAIController` self))
  (message `/Game/Game/Blueprints/iAI.iActiveNewAi` _returnvalue `Ai Class` `Ai Tree` `Ai Tb`))

(event `/Game/Game/Blueprints/Human.iXPUp`
  (params (value :type Integer))
  (bind _summoner (`self.Summoner`))
  (`/Engine/EditorBlueprintResources/StandardMacros.IsValid` _summoner
    (:`Is Valid`
      (message `/Game/Game/Blueprints/Human.iXPUp` _summoner value)
      (set `self.SummonTimeRemainning` (+ (`self.SummonTimeRemainning`) 0.01)))))

(event `/Game/Game/Blueprints/iAnimation.iFinishAttack`
  (params (Anim :type "AnimSequenceBase Object Reference") (Num :type Integer))
  (set `self.MoveAble` true)
  (set `self.Atk` 0))

(event `/Game/Recycle/BossMonster/iMonster.iSummonAttack`
  (params (Atk :type Integer))
  (`self.SummonAttacked` Atk))

(event `/Game/Game/Blueprints/iAI.iFocusToActor`
  (params (Actor :type "Actor Object Reference"))
  (`/Engine/EditorBlueprintResources/StandardMacros.IsValid` Actor
    (:`Is Valid`
      (set `self.EmTarget` Actor)
      (`self.iFocusTarget` Actor))))

(event `/Game/Game/Blueprints/Human.iFocusTarget`
  (params (Target :type "Actor Object Reference"))
  (`/Engine/EditorBlueprintResources/StandardMacros.IsValid` Target
    (:`Is Valid`
      (`self.iAISetMission` (`self.K2_GetActorLocation` Target)))))

(event `self.ReceiveAnyDamage`
  (params (Damage :type "Float (single-precision)") (DamageType :type "DamageType Object Reference") (InstigatedBy :type "Controller Object Reference") (DamageCauser :type "Actor Object Reference"))
  (`self.ShowDamage` Damage)
  (bind _result (`self.iSameSide` DamageCauser))
  (if (not _result)
    (bind _output_get (set `self.SummonTimeRemainning` (`KismetMathLibrary.FClamp` (- (`self.SummonTimeRemainning`) 0.01))))
    (if (< _output_get 0.1)
      (`self.iUnSummon`))))

(event `/Game/Game/Blueprints/iAnimation.iFinishAnimationFall`
  (params (AnimNum :type Integer)))

(fn `CreateBBValue`
  (bind _rank (`self.Rank`))
  (bind _returnvalue (`AIBlueprintHelperLibrary.GetAIController` self))
  (`/Game/Game/Utilities/xAiUtils.xCreateGFBBData` (make `/Game/NewChuAccess/Monster_Character/Gf_StructData` (* _rank 500.0) (* _rank 100.0) (`self.K2_GetActorLocation`)) (`AIBlueprintHelperLibrary.GetBlackboard` _returnvalue)))

(fn `CreateDummyActor`
  (params (NewAnimToPlay :type "AnimationAsset Object Reference") (InLifespan :type "Float (double-precision)"))
  (returns (NewParam :type Boolean) (ReturnValue :type "SkeletalMeshActor Object Reference"))
  (bind _mesh (`self.Mesh`))
  (bind _returnvalue (`|SpawnActorFromClass` "/Script/Engine.SkeletalMeshActor" (`SceneComponent.K2_GetComponentToWorld` _mesh) "AlwaysSpawn" "OverrideRootScale"))
  (bind _skeletalmeshcomponent (`SkeletalMeshActor.SkeletalMeshComponent` _returnvalue))
  (`SkinnedMeshComponent.SetSkinnedAssetAndUpdate` _skeletalmeshcomponent (`SkinnedMeshComponent.SkeletalMesh` _mesh) true)
  (`PrimitiveComponent.SetMaterial` _skeletalmeshcomponent 0 (`PrimitiveComponent.GetMaterial` _mesh 0))
  (`SkeletalMeshComponent.PlayAnimation` _skeletalmeshcomponent NewAnimToPlay false)
  (`self.SetLifeSpan` _returnvalue InLifespan)
  (return true _returnvalue))

(fn `GetBlackBoard`
  (returns (Success :type Boolean) (Blackboard :type "BlackboardComponent Object Reference") (AiControler :type "AIController Object Reference"))
  (bind _returnvalue (`AIBlueprintHelperLibrary.GetAIController` self))
  (return true (`AIController.Blackboard` _returnvalue) _returnvalue))

(fn `GetSkillData`
  (params (Atk :type Integer) (GType :type Integer))
  (returns (Found :type Boolean) (`Out Row` :type "/Game/NewChuAccess/Monster_Character/Gf_SkillStruct Structure"))
  (bind _outrownames (`DataTableFunctionLibrary.GetDataTableRowNames` "/Game/NewChuAccess/Monster_Character/GfTableSkill.GfTableSkill"))
  (for _array_element _outrownames
    (bind _returnvalue (`|GetDataTableRow` "/Game/NewChuAccess/Monster_Character/GfTableSkill.GfTableSkill" _array_element)
      (:`then`
        (bind (_affectdist _radius _damage _atk _gftype) (break `/Game/NewChuAccess/Monster_Character/Gf_SkillStruct` _returnvalue))
        (if (and (== Atk _atk) (== _gftype GType))
          (return true _returnvalue)))))
  (return false))

(fn `GetSteeringValue`
  (params (FromLoc :type "Vector Structure"))
  (returns (Success :type Boolean) (ReturnValue :type "Float (double-precision)"))
  (bind _direction (`/Game/common/GXFuncs_v9.xDirection` (`self.K2_GetActorLocation`) FromLoc))
  (bind _returnvalue (`KismetMathLibrary.Dot_VectorVector` (`KismetMathLibrary.Normal` (* _direction (1.0 1.0 0.0))) (`self.GetActorRightVector`)))
  (return (not (`KismetMathLibrary.NearlyEqual_FloatFloat` _returnvalue)) _returnvalue))

(fn `iCheckControled`
  (params (A :type "Actor Object Reference"))
  (returns (Result :type Boolean) (Current :type "Actor Object Reference"))
  (bind _summoner (`self.Summoner`))
  (`/Engine/EditorBlueprintResources/StandardMacros.IsValid` A
    (:`Is Valid`
      (return (== A _summoner) A))
    (:`Is Not Valid`
      (return (`KismetSystemLibrary.IsValid` _summoner) _summoner))))

(fn `iCurrentAnim`
  (returns (Anim :type "AnimSequenceBase Object Reference") (Value :type "Float (double-precision)"))
  (return null 0.0))

(fn `iCurrentTarget`
  (returns (Actor :type "Actor Object Reference") (Available :type Boolean))
  (bind _emtarget (`self.EmTarget`))
  (return _emtarget (`KismetSystemLibrary.IsValid` _emtarget)))

(fn `iDetectEnemy`
  (params (Max :type "Float (double-precision)") (Min :type "Float (double-precision)") (ByClass :type "Actor Class Reference") (Stat :type "/Game/NewChuAccess/Monster_Character/EEnemyStat Enum" :default "NewEnumerator0"))
  (returns (Actors :type "Array of Actor Object Reference"))
  (bind _outactors (`GameplayStatics.GetAllActorsOfClass` ByClass))
  (bind _enemies (`/Game/NewChuAccess/Bp/CDT_Utils.xDetectEnemy` ByClass Stat _outactors "/Game/Game/Blueprints/Human.Human_C" self Max Min))
  (return _enemies))

(fn `iGetAnimMesh`
  (returns (Mesh :type "SkeletalMeshComponent Object Reference"))
  (return (`self.Mesh`)))

(fn `iGetMissionStat`
  (returns (NewParam :type "/Game/Game/AITree/EMissionStatus Enum"))
  (return "NewEnumerator0"))

(fn `iGetTarget`
  (returns (Target :type "Actor Object Reference") (Available :type Boolean))
  (bind _emtarget (`self.EmTarget`))
  (return _emtarget (`KismetSystemLibrary.IsValid` _emtarget)))

(fn `iLostTarget`
  (returns (Died :type Boolean) (Faraway :type Boolean))
  (bind _emtarget (`self.EmTarget`))
  (bind _result (message `/Game/Game/Blueprints/Human.iisDied` _emtarget))
  (return _result (`KismetSystemLibrary.IsValid` _emtarget)))

(fn `ireachGoal`
  (params (Dist :type "Float (double-precision)"))
  (returns (NewParam :type Boolean))
  (bind _returnvalue (`/Game/Game/Utilities/xAiUtils.xGetBBVectorValue` "NewEnumerator0" (`AIBlueprintHelperLibrary.GetBlackboard` (`self.GetController`))))
  (bind _direction (`/Game/NewChuAccess/Bp/MX_LibA.Mx_DirectionToLocation` _returnvalue))
  (return (< (`KismetMathLibrary.VSize` (* _direction (1.0 1.0 0.0))) (* (`self.Rank`) Dist))))

(fn `iTrackToActor`
  (params (Actor :type "Actor Object Reference") (Dist :type "Float (double-precision)"))
  (returns (Closed :type Boolean))
  (return false))

(fn `LinkToSummoner`
  (bind _returnvalue (`self.K2_GetActorLocation`))
  (bind _summoner (`self.Summoner`))
  (bind _p_link (`self.P_link`))
  (bind _returnvalue_2 (`self.K2_GetActorLocation` _summoner))
  (`/Engine/EditorBlueprintResources/StandardMacros.IsValid` _summoner
    (:`Is Valid`
      (`ParticleSystemComponent.SetTemplate` _p_link "/Game/InfinityBladeEffects/Effects/FX_Mobile/combat/P_Charge_Target_Beam_Ribbon2.P_Charge_Target_Beam_Ribbon2")
      (`ParticleSystemComponent.SetBeamSourcePoint` _p_link 1 _returnvalue_2 0)
      (`ParticleSystemComponent.SetBeamTargetPoint` _p_link 1 _returnvalue 0)
      (bind (_direction _dist) (`/Game/common/GXFuncs_v9.xDirection` _returnvalue_2 _returnvalue))
      (if (> _dist 1000.0)
        (`self.iAISetMission` _returnvalue_2)))
    (:`Is Not Valid`
      (`ParticleSystemComponent.SetTemplate` (`self.P_link`) "/Game/ParticleSystem/PaticularEffect/Effects/Aura/P_AuraCircle_Temp.P_AuraCircle_Temp"))))

(fn `ProcessSummonTime`
  (bind _summontimeremainning (`self.SummonTimeRemainning`))
  (if (`self.Activated`)
    (set `self.SummonTimeRemainning` (+ _summontimeremainning -0.01))
    (else
      (set `self.SummonTimeRemainning` (+ _summontimeremainning 0.01)))))

(fn `ShowDamage`
  (params (Damage :type "Float (double-precision)"))
  (message `/Game/MenuWidget/iWidget.iShowText` (`WidgetComponent.GetUserWidgetObject` (`self.WgShowDamage`)) (`KismetStringLibrary.Conv_IntToString` (`KismetMathLibrary.FTrunc` Damage)) ""))

(fn `SummonAttacked`
  (params (Atk :type Integer))
  (returns (NewParam :type Boolean))
  (bind _returnvalue (`KismetMathLibrary.MakeVector` 0.0 0.0 -1000.0))
  (bind _rank (`self.Rank`))
  (`MovementComponent.StopMovementImmediately` (`self.CharacterMovement`))
  (set `self.MoveAble` false)
  (bind _output_get (set `self.Atk` Atk))
  (bind (_found _out_row) (`self.GetSkillData` _output_get (`self.Gdtype`)))
  (if _found
    (bind (_affectdist _radius _damage _atk _gftype _effector) (break `/Game/NewChuAccess/Monster_Character/Gf_SkillStruct` _out_row))
    (bind _returnvalue_2 (* _damage _rank))
    (bind _returnvalue_3 (* _rank _radius))
    (`|SpawnActorFromClass` "/Game/MainCharater/Weapon/Bp/Wk_Air_Blast.Wk_Air_Blast_C" (`KismetMathLibrary.Conv_VectorToTransform` (`self.K2_GetActorLocation`)) "AlwaysSpawn" "OverrideRootScale" null _returnvalue_2 _returnvalue_3 0.1)
    (`GameplayStatics.ApplyDamage` (`self.EmTarget`) _returnvalue_2 null self "/Script/Engine.DamageType")
    (bind _outactors (`GameplayStatics.GetAllActorsOfClass` "/Script/Engine.Pawn"))
    (bind (_result _sucssess) (`/Game/NewChuAccess/Bp/CDT_Utils.xNearestActor` _outactors self _returnvalue_3))
    (if _sucssess
      (for _array_element _result
        (bind _result_2 (`self.iSameSide` _array_element))
        (if (not _result_2)
          (`GameplayStatics.ApplyDamage` _array_element (* _returnvalue_2 0.1) null self "/Script/Engine.DamageType")
          (`/Game/common/GXFuncs_v9.Projectile` _effector 111.0 _returnvalue_2 111.0 self (- (`self.K2_GetActorLocation` _array_element) _returnvalue) _returnvalue _array_element true (`KismetMathLibrary.Conv_DoubleToVector` (`self.Rank`))))))
    (return true)
    (else
      (set `self.MoveAble` true)
      (return false))))

(fn `SummonDisapear`
  (params (Visible :type Boolean))
  (bind _wgtimeremain (`self.WgTimeRemain`))
  (bind _p_link (`self.P_link`))
  (`self.SummonEffect` Visible)
  (if Visible
    (`/Game/NewChuAccess/Bp/MX_LibA.Mx_DisableActor` true true true true)
    (`SceneComponent.SetHiddenInGame` _wgtimeremain false false)
    (`SceneComponent.SetHiddenInGame` _p_link false false)
    (bind _returnvalue (`AIBlueprintHelperLibrary.GetAIController` self))
    (`/Engine/EditorBlueprintResources/StandardMacros.IsValid` _returnvalue
      (:`Is Valid`
        (`self.SetActorTickEnabled` _returnvalue true)
        (set `self.Activated` true)))
    (else
      (`/Game/NewChuAccess/Bp/MX_LibA.Mx_DisableActor` false false false false true)
      (`SceneComponent.SetHiddenInGame` _wgtimeremain true false)
      (`SceneComponent.SetHiddenInGame` _p_link true false)
      (bind _returnvalue_2 (`AIBlueprintHelperLibrary.GetAIController` self))
      (`/Engine/EditorBlueprintResources/StandardMacros.IsValid` _returnvalue_2
        (:`Is Valid`
          (`self.SetActorTickEnabled` _returnvalue_2 false)
          (set `self.Activated` false))))))

(fn `SummonEffect`
  (params (Showing :type Boolean)))

(fn `UpdateBlackBoard`
  (bind (_success _blackboard) (`self.GetBlackBoard`))
  (`/Game/Game/Utilities/xAiUtils.xGetBBActorValue` "NewEnumerator1" _blackboard (`self.Summoner`) true))

(fn `UserConstructionScript`
  (`parent.UserConstructionScript`)
  (`self.iChooseTypeAndSign` (`self.Gdtype`) (`self.GfSign`)))